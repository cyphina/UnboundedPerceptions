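; RTS game mode that manages streamed level switching and reacts to section completion.
; On BeginPlay it caches the RTS game instance and binds to the EventManager, whose completion delegate spawns a next-section effect widget.
; StreamLevelAsync shows a loading widget, saves and unloads the current level, then unpauses, streams in the requested one, restores its data through the game instance and notifies the widget.
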(event Custom|OnSectionCompleted
  (params (sectionName :type Gameplay%20Tag%20Structure))
  (bind _returnvalue (UserInterface|CreateWidget "/Game/RTS_Tutorial/HUDs/MainUI/NextSectionEffectWidget.NextSectionEffectWidget_C" 0 (Variables|Default|GeteventManager)))
  (UserInterface|Viewport|AddtoViewport _returnvalue 1))

(event EventBeginPlay
  (|CallParentFunction)
  (EventDispatchers|AssignOnSectionCompletedDelegate (Variables|Default|GeteventManager) (delegate Custom|OnSectionCompleted))
  (bind _asrtsgame_instance (Utilities|Casting|CastToRTSGameInstance (Game|GetGameInstance)))
  (Variables|Default|SetgameInstanceRef _asrtsgame_instance))

(event EventStreamLevelAsync
  (params (levelName :type Name :default "None"))
  (bind _returnvalue (UserInterface|CreateWidget "/Game/RTS_Tutorial/HUDs/Loading/BPLoadingWidget.BPLoadingWidget_C"))
  (UserInterface|Viewport|AddtoViewport _returnvalue 10)
  (if (Utilities|Name|NotEqual(Name) (Utilities|String|StringToName (Variables|Default|GetcurrentLevelName)) "None")
    (Class|MyGameInstance|SaveLevelData (Variables|Default|GetgameInstanceRef) (Utilities|String|StringToName (Variables|Default|GetcurrentLevelName)))
    (Game|UnloadStreamLevel(byName) (Utilities|String|StringToName (Variables|Default|GetcurrentLevelName)) false))
  (if (Utilities|Name|NotEqual(Name) levelName "None")
    (Game|SetGamePaused false)
    (Game|LoadStreamLevel(byName) levelName true)
    (bind _output_get (Variables|Default|SetcurrentLevelName (Utilities|String|ToString(Name) levelName)))
    (Class|MyGameInstance|LoadLevelData (Variables|Default|GetgameInstanceRef) (Utilities|String|StringToName _output_get))
    (Class|LoadingWidget|OnLoadingFinished _returnvalue)))

(fn ConstructionScript)