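; CameraPawnController is the RTS player controller for the camera pawn, handling cursor hit tests, hero tab-selection, screen-edge panning and building placement.
; BeginPlay spawns the construction manager and ghost building, which follows the cursor in build mode and rotates on input.
; Outside the starting level, a looping timer gathers objects overlapping heroes and toggles their fade components to hide or restore them.
; It also seeds dialog topics and carries debug keys for quest completion and screen fades.
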(event Custom|ScreenFade
  ;[1 0.2334 0.7802] Debugging HUD Stuff
  ;;[1 1 1] Debug FadeIn
  (bind _newtrack_0 (Timeline|FadeScreenTimeline ReverseFromEnd)
    (:Update
      (Rendering|Material|SetScalarParameterValue "/Game/RTS_Tutorial/Materials/UIMats/TransitionMat/amount_paraCollection.amount_paraCollection" "amount" _newtrack_0 :!class /Script/Engine.KismetMaterialLibrary))))

(event EventBeginPlay
  ;[0 0 0] This is where all the things that pertain to starting up the game go
  (Utilities|FlowControl|Sequence
    (:then_0
      (|CallParentFunction))
    (:then_1
      (Utilities|SetupConstructionStuff (Math|Transform|MakeTransform "0, 0, 0")))
    (:then_2
      (bind _asbp_rtspawn (Utilities|Casting|CastToBP_RTSPawn (Class|UserInput|GetCameraPawn)))
      (Variables|Default|SetBPPawn _asbp_rtspawn))
    (:then_3
      (bind _returnvalue (Game|GetCurrentLevelName true)) ; If we're not on starting level
      (bind _asmy_rtsgame_mode (Utilities|Casting|CastToMyRTSGameMode (Game|GetGameMode)))
      (if (Utilities|Enum|NotEqual(Enum) _returnvalue (Class|RTSGameMode|GetStartingLvlName _asmy_rtsgame_mode))
        (bind _returnvalue_2 (Utilities|Time|SetTimerbyFunctionName 0 "UpdateFadeActors" 0.1 true)) ; Setup a timer so we don't have to constantly check update
        (Variables|Default|SettimerHandleFade _returnvalue_2)))
    (:then_4
      (Utilities|InitDialogTopics)
      (bind _returnvalue_3 (Rendering|Material|CreateDynamicMaterialInstance "/Game/RTS_Tutorial/Particles/LavenderRain/Ripple.Ripple" "None" :!class /Script/Engine.KismetMaterialLibrary))
      (Variables|Default|SetDecalMaterial _returnvalue_3))))

(event EventTick
  (params (DeltaSeconds :type Float%20%28single-precision%29))
  ;[1 1 1] Tick
  (Utilities|FlowControl|Sequence
    (:then_0
      (if (Variables|Building|GetbuildModeActive)
        (|SetCursorWorldPosition)))
    (:then_1
      (|CallParentFunction DeltaSeconds))))

(event Input|ActionEvents|InputActionRightClick
  (params (Key :type Key%20Structure :default "None"))
  ;[1 1 1] Get out of Building Mode
)

(event Input|ActionEvents|InputActionRotateBuildingLeft
  (params (Key :type Key%20Structure :default "None"))
  (bind _ghostbuildingref (Variables|References|GetGhostBuildingRef))
  (bind _returnvalue (Transformation|GetActorRotation _ghostbuildingref))
  (bind (_roll _pitch _yaw) (Math|Rotator|BreakRotator _returnvalue))
  ;[1 1 1] Building Rotation
  (:Pressed
    (if (and (Variables|Building|GetbuildModeActive) (Utilities|IsValid _ghostbuildingref))
      (Transformation|SetActorRotation _ghostbuildingref (Math|Rotator|MakeRotator _roll _pitch (- _yaw (Variables|Building|GetbuildRotationRate)))))))

(event Input|ActionEvents|InputActionRotateBuildingRight
  (params (Key :type Key%20Structure :default "None"))
  (bind _ghostbuildingref (Variables|References|GetGhostBuildingRef))
  (bind _returnvalue (Transformation|GetActorRotation _ghostbuildingref))
  (bind (_roll _pitch _yaw) (Math|Rotator|BreakRotator _returnvalue))
  ;[1 1 1] Building Rotation
  (:Pressed
    (if (and (Variables|Building|GetbuildModeActive) (Utilities|IsValid _ghostbuildingref))
      (Transformation|SetActorRotation _ghostbuildingref (Math|Rotator|MakeRotator _roll _pitch (+ _yaw (Variables|Building|GetbuildRotationRate)))))))

(event Input|KeyboardEvents|J
  (params (Key :type Key%20Structure :default "None"))
  (bind _returnvalue (Class|UserInput|GetGameMode))
  (bind _questmanager (Variables|/Script/MyProject.RTSGameMode|GetquestManager _returnvalue))
  (bind _quests (Variables|/Script/MyProject.QuestManager|Getquests _questmanager))
  (bind _output (Utilities|Array|Get(acopy) _quests))
  ;[1 0.2334 0.7802] Debugging HUD Stuff
  ;;[1 1 1] Debug Complete Quest Subgoal
  (:Pressed
    (Utilities|IsValid _output
      (:Is%20Valid
        (Class|Quest|CompleteSubGoal _output 0 false)))))

(event Input|KeyboardEvents|O
  (params (Key :type Key%20Structure :default "None"))
  ;[1 0.2334 0.7802] Debugging HUD Stuff
  ;;[1 1 1] Debug FadeIn
  (:Pressed
    (Utilities|FlowControl|FlipFlop
      (:A
        (bind _newtrack_0 (Timeline|FadeScreenTimeline PlayFromStart)
          (:Update
            (Rendering|Material|SetScalarParameterValue "/Game/RTS_Tutorial/Materials/UIMats/TransitionMat/amount_paraCollection.amount_paraCollection" "amount" _newtrack_0 :!class /Script/Engine.KismetMaterialLibrary))))
      (:B
        (Timeline|FadeScreenTimeline ReverseFromEnd)))))

(event Input|KeyboardEvents|Z
  (params (Key :type Key%20Structure :default "None"))
  ;[1 0.2334 0.7802] Debugging HUD Stuff
  ;;[0.5503 0.8996 1] Add Some EXP
)

(fn ConstructionScript)

(fn IsRect
  (bind _startmouseposition (Variables|Mouse|GetstartMousePosition))
  (bind _endmouseposition (Variables|Mouse|GetendMousePosition))
  (bind _returnvalue (- _startmouseposition _endmouseposition))
  (return (> (Math|Float|Sqrt (Math|Vector2D|DotProduct(2D) _returnvalue _returnvalue)) 1e+01)))

(fn GetHitObjectActor
  (bind (_worldlocation _worlddirection) (Game|Player|ConvertMouseLocationToWorldSpace))
  (bind _outhit (Collision|LineTraceForObjects _worldlocation (+ _worldlocation (* _worlddirection (* (Variables|Camera|GetmaxArmDistance) 3.0))) (Utilities|Array|MakeArray "ObjectTypeQuery7" "ObjectTypeQuery12" "ObjectTypeQuery1" "ObjectTypeQuery8" "ObjectTypeQuery9") false 0 "None"))
  (if (!= (.HitActor (Collision|BreakHitResult _outhit)) 0)
    (return (.HitActor (Collision|BreakHitResult _outhit)))
    (else
      (return 0))))

(fn UpdateFadeActors
  (Utilities|Array|Clear (Variables|Fade|GethitMeshes))
  (bind _array_element (Utilities|HeroLoop :!label _label)
    (:LoopBody
      (if (Utilities|IsValid _array_element)
        (bind (_hits _returnvalue) (Class|Ally|GetOverlappingObjects _array_element))
        (if _returnvalue
          (for _array_element_2 _hits
            (if (Utilities|IsValidClass (Utilities|GetClass (.HitActor (Collision|BreakHitResult _array_element_2))))
              (if (!= (Actor|GetComponentbyClass (.HitActor (Collision|BreakHitResult _array_element_2)) "/Game/RTS_Tutorial/Blueprints/Effects/Fade/BP_FadeComponent.BP_FadeComponent_C") 0)
                (Utilities|Array|AddUnique (Variables|Fade|GethitMeshes) (.HitActor (Collision|BreakHitResult _array_element_2))) ; Generate list of hit meshes for all units
              ))))
        (else
          (goto _label Break))))
    (:Completed
      (Fade|SetShownMeshes) ; Look at our list of already hidden meshes\nand if any of them are not hit anymore, then\nthey are now visible
      (Fade|SetHiddenMeshes) ; Create a list of all meshes that are hidden
    )))

(fn SetShownMeshes
  ;[1 1 1] For each mesh, set each mesh to Not Hidden.  This is done when leaving a hidden mesh, so we have to check to see the tick when the hit mesh is finally not in hidden meshes.  We keep track of the hidden meshes so once the hit meshes don't correspond to hidden, we make it visible again
  (for _array_element (Variables|Fade|GethiddenMeshes)
    (if (not (Utilities|Array|ContainsItem (Variables|Fade|GethitMeshes) _array_element))
      (if (!= (Actor|GetComponentbyClass _array_element "/Game/RTS_Tutorial/Blueprints/Effects/Fade/BP_FadeComponent.BP_FadeComponent_C") 0) ; Some kind of null reference here not sure why
        (Default|ToggleHideMesh (Actor|GetComponentbyClass _array_element "/Game/RTS_Tutorial/Blueprints/Effects/Fade/BP_FadeComponent.BP_FadeComponent_C") false)))))

(fn SetHiddenMeshes
  ;[1 1 1] For each component, go set each mesh to "HIDDEN"
  (bind _output_get (Variables|Fade|SethiddenMeshes (Variables|Fade|GethitMeshes)))
  (for _array_element _output_get
    (if (!= 0 (Utilities|GetClass (Actor|GetComponentbyClass _array_element "/Game/RTS_Tutorial/Blueprints/Effects/Fade/BP_FadeComponent.BP_FadeComponent_C")))
      (Default|ToggleHideMesh (Actor|GetComponentbyClass _array_element "/Game/RTS_Tutorial/Blueprints/Effects/Fade/BP_FadeComponent.BP_FadeComponent_C") true))))

(fn GetHitObjectType
  (bind _array (Utilities|Array|MakeArray "ObjectTypeQuery9" "ObjectTypeQuery7" "ObjectTypeQuery8" "ObjectTypeQuery2" "ObjectTypeQuery1" "ObjectTypeQuery11" "ObjectTypeQuery13"))
  (bind _hitresult (Class|PlayerController|GetHitResultUnderCursorforObjects _array true))
  (bind (_bblockinghit _binitialoverlap _time _distance _location _impactpoint _normal _impactnormal _physmat _hitactor _hitcomponent) (Collision|BreakHitResult _hitresult))
  (bind _returnvalue (!= _hitactor 0))
  (if _returnvalue
    (return (Collision|GetCollisionObjectType _hitcomponent) _returnvalue)
    (else
      (return "ECC_WorldStatic" false))))

(fn CheckClosestHero
  (for _array_element (Variables|/Script/MyProject.BasePlayer|GetselectedHeroes (Variables|Default|GetbasePlayer))
    (if (< (Math|Vector|DotProduct (- (Transformation|GetActorLocation (Raycasting|GetHitObjectActor)) (Transformation|GetActorLocation _array_element)) (- (Transformation|GetActorLocation (Raycasting|GetHitObjectActor)) (Transformation|GetActorLocation _array_element))) (LocalVariables|GetclosestSqrDistance))
      (LocalVariables|SetclosestSqrDistance (Math|Vector|DotProduct (- (Transformation|GetActorLocation (Raycasting|GetHitObjectActor)) (Transformation|GetActorLocation _array_element)) (- (Transformation|GetActorLocation (Raycasting|GetHitObjectActor)) (Transformation|GetActorLocation _array_element))))
      (LocalVariables|SetclosestHero _array_element)
      (return (LocalVariables|GetclosestHero))))
  (return (LocalVariables|GetclosestHero)))

(fn TabHeroSelected
  (bind _baseplayer (Variables|Default|GetbasePlayer))
  (bind _baseplayer_2 (Variables|Default|GetbasePlayer))
  (bind _selectedallies (Variables|/Script/MyProject.BasePlayer|GetselectedAllies _baseplayer_2))
  (bind _returnvalue (Utilities|Array|Length _selectedallies))
  (if (> _returnvalue 1) ; Do we have more than one unit selected
    ;[1 1 1] Tab through selected allies
    (bind _output_get (Variables|/Script/MyProject.BasePlayer|SetunitIndex _baseplayer_2 (select (== (Variables|/Script/MyProject.BasePlayer|GetunitIndex _baseplayer_2) (Utilities|Array|LastIndex _selectedallies)) 0 (+ (Variables|/Script/MyProject.BasePlayer|GetunitIndex _baseplayer_2) 1))))
    (Class|ActionbarInterface|SingleAllyViewIndexFree (Class|HUDManager|GetActionHUD (Class|UserInput|GetHUDManager)) (Utilities|Array|Get(acopy) _selectedallies _output_get))
    (else
      ;[1 1 1] Tab through heroes if no hero is selected
      (if (> _returnvalue 0) ; If only one unit selected, tab through heroes
        (bind _output_get_2 (LocalVariables|SetselectedHeroIndex (Variables|/Script/MyProject.BaseHero|GetheroIndex (Utilities|Array|Get(acopy) (Variables|/Script/MyProject.BasePlayer|GetselectedHeroes _baseplayer))))) ; Tab through all the heroes by order in hero array\nSet to -1 by default
        (Class|Unit|SetSelected (Utilities|Array|Get(acopy) (Variables|/Script/MyProject.BasePlayer|Getheroes _baseplayer) (select (== _output_get_2 (Utilities|Array|LastIndex (Variables|/Script/MyProject.BasePlayer|Getheroes _baseplayer))) 0 (+ _output_get_2 1))) false))
      (Class|Unit|SetSelected (Utilities|Array|Get(acopy) (Variables|/Script/MyProject.BasePlayer|Getheroes _baseplayer) (select (== _output_get_2 (Utilities|Array|LastIndex (Variables|/Script/MyProject.BasePlayer|Getheroes _baseplayer))) 0 (+ _output_get_2 1))) true))))

(fn PauseTimedFunctions
  (Utilities|Time|PauseTimerbyHandle (Variables|Default|GettimerHandleFade)))

(fn UnpauseTimedFunctions
  (Utilities|Time|UnpauseTimerbyHandle (Variables|Default|GettimerHandleFade)))