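; Construction proxy that stands in for a building under construction, showing its mesh in a ghost material.
; While any workers are reported in, Tick advances a clock scaled by game speed, regardless of crew size.
; At the construction time it broadcasts completion, runs worker release, removes its HUD and destroys itself.
; A HUD request for this actor lerps the camera to it and shows the proxy HUD, disabling the main one.
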(event Custom|DisplayHUD
  (params (actor :type Actor%20Object%20Reference))
  (bind _controllerref (Variables|Default|GetControllerRef))
  ;[1 1 1] Is this actor selecting me?
  (if (== actor self)
    (Utilities|FlowControl|Sequence
      (:then_0
        ;;[1 1 1] Camera Move to Selected
        (bind _newlocation (|LerpLocation)
          (:Update
            (Transformation|SetActorLocation (Variables|/Game/RTS_Tutorial/Blueprints/CameraPawnController.CameraPawnController_C|GetCameraPawnRef (Variables|Default|GetControllerRef)) _newlocation false false))))
      (:then_1
        (UserInterface|Viewport|AddtoViewport (Variables|Default|GetproxyHUD) 0)
        (Input|SetInputModeUIOnly _controllerref 0 "LockOnCapture")
        (Widget|SetIsEnabled (Class|HUDManager|GetMainHUD (Default|GetHudManager _controllerref)) false)))))

(event Custom|AdjustTime
  (params (timeMultiplier :type Float%20%28single-precision%29))
  (Variables|Time|SettimeUnit timeMultiplier))

(event EventTick
  (params (DeltaSeconds :type Float%20%28single-precision%29))
  (bind _proxyhud (Variables|Default|GetproxyHUD))
  (Variables|Time|Setdelta DeltaSeconds)
  (if (not (Variables|Default|GetisConstructionCompleted))
    (CallFunction|DoWork)
    (if (>= (Variables|Time|GetworkTimeSpent) (Variables|Time|GetconstructionTime))
      (Variables|Default|SetisConstructionCompleted true)
      (Default|CallConstructionCompleted self)
      (CallFunction|FinishConstruction)
      (if (UserInterface|Viewport|IsinViewport _proxyhud)
        (Default|RemoveHUD _proxyhud))
      (Utilities|FlowControl|Delay 0.2)
      (Actor|DestroyActor))))

(event EventBeginPlay
  (bind _output_get (Variables|Default|SetgameStateRef (.AsMy%20Game%20State (Utilities|Casting|CastToMyGameState (Game|GetGameState)))))
  (EventDispatchers|BindEventtoUpdateGameSpeedDelegate _output_get (EventDispatchers|CreateEvent :!event Custom|AdjustTime))
  (Variables|Time|SettimeUnit (Variables|/Script/MyProject.RTSGameState|GetspeedModifier (Variables|Default|GetgameStateRef)))
  (bind _ascamera_pawn_controller (Utilities|Casting|CastToCameraPawnController (Game|GetPlayerController 0)))
  (bind _output_get_2 (Variables|Default|SetcontrollerRef _ascamera_pawn_controller))
  (EventDispatchers|BindEventtoHUDRequest _output_get_2 (EventDispatchers|CreateEvent :!event Custom|DisplayHUD))
  (bind _returnvalue (UserInterface|CreateWidget "/Game/RTS_Tutorial/HUDs/BuildingUI/Proxy_HUD.Proxy_HUD_C" 0 self (Variables|Default|GetcontrollerRef)))
  (Variables|Default|SetproxyHUD _returnvalue))

(fn ConstructionScript
  (bind _staticmesh (Variables|Default|GetStaticMesh))
  (Components|StaticMesh|SetStaticMesh _staticmesh (Variables|Default|GetdisplayMesh))
  (Rendering|Material|SetMaterial _staticmesh 0 "/Game/RTS_Tutorial/Materials/Ghost_M_Inst.Ghost_M_Inst")
  (CallFunction|SetBuildingEntrance (Variables|Default|GetEntrance) (Variables|Default|GetStaticMesh))
  (CallFunction|SetBuildingCollisionBox (Variables|Default|GetCollision) (Variables|Default|GetStaticMesh)))

(fn SetConstructionTime
  (params (workHours :type Float%20%28single-precision%29))
  (Variables|Time|SetconstructionTime (* workHours 6e+01))
  (return))

(fn DoWork
  ;[1 1 1] If we have someone working on the building, setup the timer
  (if (> (CallFunction|GetWorkForce) 0.0)
    (bind _output_get (Variables|Time|SetclockWork (.clockWorkOut (CallFunction|SetClockwork (Variables|Time|Getdelta) (Variables|Time|GettimeUnit) (Variables|Time|GetclockWork)))))
    (Variables|Time|SetworkTimeSpent _output_get)
    (return)))

(fn GetWorkForce
  (return (Math|Conversions|ToFloat(Integer) (Utilities|Array|Length (Variables|Default|GetactiveWorkers)))))

(fn ReporttoShift
  (params (worker :type Construction%20Worker%20BP%20Object%20Reference))
  (Utilities|Array|Add (Variables|Default|GetactiveWorkers) worker)
  (return))

(fn FinishConstruction
  (if (> (CallFunction|GetWorkForce) 0.0)
    (for _array_element (Variables|Default|GetactiveWorkers)
      (Default|SetIsBusy _array_element false)
      (Rendering|SetActorHiddenInGame _array_element false)
      (return))
    (Variables|Default|SetactiveWorkers (Utilities|Array|MakeArray 0)) ; Clear Array
    (return)
    (else
      (return))))

(fn GetProxyName)