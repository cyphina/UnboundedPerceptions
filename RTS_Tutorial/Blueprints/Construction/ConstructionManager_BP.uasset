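; Construction manager actor for the RTS that turns queued build orders into finished buildings.
; Queuing an order spawns a construction proxy with the building's display mesh and required work hours, stored in parallel proxy and config arrays.
; When a proxy's completion dispatcher fires, the manager removes its entries, spawns the configured building class at the saved transform and destroys the proxy.
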(event Custom|BindConstructionComplete
  (params (Proxy :type Construction%20Proxy%20BP%20Object%20Reference))
  ;[1 0.3356 0.7917] Binds Event to Proxy's Event Dispatcher
  (EventDispatchers|BindEventtoConstructionCompleted Proxy (EventDispatchers|CreateEvent :!event Custom|ConstructionCompleted)))

(event Custom|ConstructionCompleted
  (params (Proxy :type Construction%20Proxy%20BP%20Object%20Reference))
  (CallFunction|FinishConstruction Proxy))

(fn ConstructionScript)

(fn QueueConstruction
  (params (ConstructionStruct :type Construction%20Struct%20Structure))
  (bind (_buildingclass _transform _displaymesh _workhoursrequired) (Utilities|Struct|BreakConstruction_Struct ConstructionStruct))
  (bind _returnvalue (Game|SpawnActorfromClass "/Game/RTS_Tutorial/Blueprints/Construction/ConstructionProxy_BP.ConstructionProxy_BP_C" _transform "AlwaysSpawn" 0 _displaymesh 0))
  (CallFunction|BindConstructionComplete _returnvalue)
  (Utilities|Array|Add (Variables|Default|GetProxies) _returnvalue)
  (Utilities|Array|Add (Variables|Default|GetQueue) ConstructionStruct)
  (Default|SetConstructionTime _returnvalue _workhoursrequired))

(fn FinishConstruction
  (params (Proxy :type Construction%20Proxy%20BP%20Object%20Reference))
  (bind _proxies (Variables|Default|GetProxies))
  (bind _queue (Variables|Default|GetQueue))
  (bind _output_get (LocalVariables|Setindex (Utilities|Array|FindItem _proxies Proxy)))
  (LocalVariables|Setconfig (Utilities|Array|Get(acopy) _queue _output_get))
  (Utilities|Array|RemoveIndex _queue (LocalVariables|Getindex))
  (Utilities|Array|RemoveIndex _proxies (LocalVariables|Getindex))
  (Game|SpawnActorfromClass (.BuildingClass (Utilities|Struct|BreakConstruction_Struct (LocalVariables|Getconfig))) (.Transform (Utilities|Struct|BreakConstruction_Struct (LocalVariables|Getconfig))) "Undefined" 0 0 0)
  (Actor|DestroyActor Proxy))