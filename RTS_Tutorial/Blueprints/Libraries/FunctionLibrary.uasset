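; Function library of shared helpers for the RTS game, covering cursor, building, time and group math.
; Cursor deprojection plus a line trace yields world positions, and GridSnap rounds an axis to the nearest grid step.
; Building helpers place collision boxes and entrances from mesh local bounds.
; SetClockwork accumulates scaled time wrapped at one day, HUDLerp wraps a vector lerp, and center-point functions average XY locations of actors or first-player allies.
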(fn GetCursorWorldPosition
  (params (Controller :type Player%20Controller%20Object%20Reference) (SightDistance :type Float%20%28single-precision%29))
  (bind (_worldlocation _worlddirection) (Game|Player|ConvertMouseLocationToWorldSpace Controller))
  (bind _outhit (Collision|LineTraceByChannel 0 _worldlocation (+ _worldlocation (* _worlddirection SightDistance)) "TraceTypeQuery3" false 0 "None"))
  (return (.Location (Collision|BreakHitResult _outhit))))

(fn GridSnap
  (params (Axis :type Float%20%28single-precision%29) (Grid%20Size :type Integer))
  (return (Math|Conversions|ToFloat(Integer) (* (Math|Float|Floor (/ (+ Axis (Math|Conversions|ToFloat(Integer) (/ Grid%20Size 2))) (Math|Conversions|ToFloat(Integer) Grid%20Size))) Grid%20Size))))

(fn SetClockwork
  (params (deltaSeconds :type Float%20%28single-precision%29) (TimeMultiplier :type Float%20%28single-precision%29) (Clockwork%20In :type Float%20%28single-precision%29))
  (bind _returnvalue (* deltaSeconds TimeMultiplier))
  (bind _returnvalue_2 (+ _returnvalue Clockwork%20In))
  (bind (_remainder _returnvalue_3) (Math|Float|Division(WholeandRemainder) _returnvalue_2 8.64e+04))
  ;[0.8699 0.6198 1] Takes in delta (how many seconds pass per frame), time unit (how long should "1 second" be), and Clockwork In (accumulator)
  (return _remainder _returnvalue_3))

(fn SetBuildingCollisionBox
  (params (collision :type Box%20Component%20Object%20Reference) (mesh :type Static%20Mesh%20Component%20Object%20Reference))
  (bind _min (Components|StaticMesh|GetLocalBounds mesh))
  (Components|Box|SetBoxExtent collision (Math|Vector|MakeVector 49.0 (- (Math|Float|Absolute(Float) (.y _min)) 1e+01) 1e+01) true)
  (Transformation|SetRelativeLocation collision (Math|Vector|MakeVector (+ (Math|Float|Absolute(Float) (.x _min)) 49.0) 0.0 1e+01) false false)
  (return))

(fn SetBuildingEntrance
  (params (Entrance :type Scene%20Component%20Object%20Reference) (Mesh :type Static%20Mesh%20Component%20Object%20Reference))
  (Transformation|SetRelativeLocation Entrance (Math|Vector|MakeVector (+ (Math|Float|Absolute(Float) (.x (.Min (Components|StaticMesh|GetLocalBounds Mesh)))) (LocalVariables|GetentranceDistance)) 0.0 0.0) false false)
  (return))

(fn HUDLerp
  (params (startDest :type Vector) (endDest :type Vector) (speed :type Float%20%28single-precision%29))
  (return (Math|Vector|Lerp(Vector) startDest endDest speed)))

(fn FindAlliesCenterPoint
  (params (WorldContext :type Object%20Object%20Reference))
  (bind _asbase_player (Utilities|Casting|CastToBasePlayer (Utilities|Array|Get(acopy) (Variables|/Script/Engine.GameStateBase|GetPlayerArray (Game|GetGameState WorldContext)))))
  (for _array_element (Variables|/Script/MyProject.BasePlayer|Getallies _asbase_player)
    (LocalVariables|SetsumX (+ (LocalVariables|GetsumX) (.x (Transformation|GetActorLocation _array_element))))
    (LocalVariables|SetsumY (+ (LocalVariables|GetsumY) (.y (Transformation|GetActorLocation _array_element)))))
  (return (Math|Vector|MakeVector (/ (LocalVariables|GetsumX) (Math|Conversions|ToFloat(Integer) (Utilities|Array|Length (Variables|/Script/MyProject.BasePlayer|Getallies _asbase_player)))) (/ (LocalVariables|GetsumY) (Math|Conversions|ToFloat(Integer) (Utilities|Array|Length (Variables|/Script/MyProject.BasePlayer|Getallies _asbase_player)))) 0.0)))

(fn FindCenterPointActors
  (params (actors :type Array%20of%20Actor%20Object%20References))
  (bind _returnvalue (Utilities|Array|Length actors))
  (for _array_element actors
    (LocalVariables|SetsumX (+ (LocalVariables|GetsumX) (.x (Transformation|GetActorLocation _array_element))))
    (LocalVariables|SetsumY (+ (LocalVariables|GetsumY) (.y (Transformation|GetActorLocation _array_element)))))
  (return (Math|Vector|MakeVector (/ (LocalVariables|GetsumX) (Math|Conversions|ToFloat(Integer) _returnvalue)) (/ (LocalVariables|GetsumY) (Math|Conversions|ToFloat(Integer) _returnvalue)) 0.0)))