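; Ice pillar spell actor that grows into place and applies a gameplay effect to actors around it.
; A RetractExpand timeline scales its height from BeginPlay, then destroys it if nearly flat or gives it the frozen material.
; Stop halts the timeline and sizes the effect sphere by current growth; leaving the sphere removes IcyPresence.
; Box overlaps on two custom channels count placement blockers, and the CanBePlaced setter swaps materials.
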(event OnComponentBeginOverlap(Box)
  (params (OverlappedComponent :type Primitive%20Component%20Object%20Reference) (OtherActor :type Actor%20Object%20Reference) (OtherComp :type Primitive%20Component%20Object%20Reference) (OtherBodyIndex :type Integer) (bFromSweep :type Boolean) (SweepResult :type Hit%20Result%20Structure%20%28by%20ref%29))
  (bind _returnvalue (Collision|GetCollisionObjectType OverlappedComponent))
  (if (not (and (Utilities|Enum|NotEqual(Enum) _returnvalue "ECC_GameTraceChannel6") (Utilities|Enum|NotEqual(Enum) _returnvalue "ECC_GameTraceChannel7")))
    (Variables|Default|SetbCanBePlaced false)
    (Math|Integer|IncrementInt (Variables|Default|GetoverlapBlockCount))))

(event OnComponentEndOverlap(Box)
  (params (OverlappedComponent :type Primitive%20Component%20Object%20Reference) (OtherActor :type Actor%20Object%20Reference) (OtherComp :type Primitive%20Component%20Object%20Reference) (OtherBodyIndex :type Integer))
  (bind _returnvalue (Collision|GetCollisionObjectType OverlappedComponent))
  (bind _overlapblockcount (Variables|Default|GetoverlapBlockCount))
  (if (not (and (Utilities|Enum|NotEqual(Enum) _returnvalue "ECC_GameTraceChannel6") (Utilities|Enum|NotEqual(Enum) _returnvalue "ECC_GameTraceChannel7")))
    (Math|Integer|DecrementInt _overlapblockcount
      (:%20%20
        (if (== _overlapblockcount 0)
          (Variables|Default|SetbCanBePlaced true))))))

(event OnComponentBeginOverlap(Sphere)
  (params (OverlappedComponent :type Primitive%20Component%20Object%20Reference) (OtherActor :type Actor%20Object%20Reference) (OtherComp :type Primitive%20Component%20Object%20Reference) (OtherBodyIndex :type Integer) (bFromSweep :type Boolean) (SweepResult :type Hit%20Result%20Structure%20%28by%20ref%29))
  (GameplayEffects|ApplyGameplayEffectSpecToSelf (Ability|GetAbilitySystemComponent OtherActor) (Variables|Default|GetgameplayEffectSpec)))

(event OnComponentEndOverlap(Sphere)
  (params (OverlappedComponent :type Primitive%20Component%20Object%20Reference) (OtherActor :type Actor%20Object%20Reference) (OtherComp :type Primitive%20Component%20Object%20Reference) (OtherBodyIndex :type Integer))
  (GameplayEffects|RemoveActiveGameplayEffectbySourceEffect (Ability|GetAbilitySystemComponent OtherActor) "/Game/RTS_Tutorial/Blueprints/SpellSystem/SpellEffect/IcyPresence.IcyPresence_C" 0 -1))

(event Custom|Expand/Retract
  (if (not (Variables|Default|GetbPlaced)) ; If this is already not placed
    (bind _icescale (Timeline|Retract/Expand Play) ; Time should match up with IcePillar channel time
      (:Update
        (Transformation|SetRelativeScale3D (Variables|Default|GetScene) (Math|Vector|MakeVector 1.5 1.5 (Math|Float|Lerp 0.0 5.0 _icescale)))
        (Variables|Default|SetbCanBePlaced true))
      (:Finished
        (if (< _icescale 0.01) ; If we retract to too small of a size kill ourselves\nwhen the animation finishes
          (Actor|DestroyActor)
          (else
            (Rendering|Material|SetMaterial (Variables|Default|GetCube) 0 "/Game/InfinityBladeIceLands/Environments/Ice/Env_Ice_Terrain/Materials/M_Env_Ice_Frozen_River_1.M_Env_Ice_Frozen_River_1")))))))

(event Custom|Stop
  (CallFunction|CreateEffectSphere (stale _icescale))
  (bind _icescale (Timeline|Retract/Expand Stop) ; Time should match up with IcePillar channel time
    (:Update
      (Transformation|SetRelativeScale3D (Variables|Default|GetScene) (Math|Vector|MakeVector 1.5 1.5 (Math|Float|Lerp 0.0 5.0 _icescale)))
      (Variables|Default|SetbCanBePlaced true))
    (:Finished
      (if (< _icescale 0.01) ; If we retract to too small of a size kill ourselves\nwhen the animation finishes
        (Actor|DestroyActor)
        (else
          (Rendering|Material|SetMaterial (Variables|Default|GetCube) 0 "/Game/InfinityBladeIceLands/Environments/Ice/Env_Ice_Terrain/Materials/M_Env_Ice_Frozen_River_1.M_Env_Ice_Frozen_River_1"))))))

(event EventBeginPlay
  (Components|Timeline|SetLooping (Variables|Default|GetRetract/Expand) false) ; We placed it, so play it once to form the actual ice pillar
  (CallFunction|Expand/Retract))

(fn ConstructionScript)

(fn SetCanbePlaced
  (params (bCanBePlaced :type Boolean))
  (bind _cube (Variables|Default|GetCube))
  (if (Variables|Default|GetbCanBePlaced)
    (if (not bCanBePlaced)
      (Rendering|Material|SetMaterial _cube 0 "/Game/RTS_Tutorial/Materials/SpellMats/IcePillar/Mat_IceBlock_Inst.Mat_IceBlock_Inst")
      (Variables|Default|SetbCanBePlaced bCanBePlaced :!label _label))
    (elif bCanBePlaced
      (Rendering|Material|SetMaterial _cube 0 "/Game/InfinityBladeEffects/Effects/FX_Materials/Misc/M_FlickerGlow_Forge_IB_INST.M_FlickerGlow_Forge_IB_INST")
      (goto _label))))

(fn CreateEffectSphere
  (params (radiusPower :type Float%20%28single-precision%29))
  (Components|Sphere|SetSphereRadius (Variables|Default|GetSphere) (* radiusPower (Variables|Default|GetsphereRadiusModifier)) true))