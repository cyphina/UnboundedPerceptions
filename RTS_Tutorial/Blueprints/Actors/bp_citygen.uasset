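; City generator actor, apparently an early draft, meant to place buildings beside a road.
; Its construction script enables query and physics collision on all its static mesh components.
; MakeSideBuilldings, not called here, walks RoadData's segments and adds a cube per TrackList entry at its rotated, scaled start tangent.
; That offset ignores each segment's position, and debug prints remain.
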(event EventBeginPlay)

(event Collision|EventActorBeginOverlap
  (params (OtherActor :type Actor%20Object%20Reference)))

(event EventTick
  (params (DeltaSeconds :type Float%20%28single-precision%29)))

(fn ConstructionScript
  (|CallParentFunction)
  (for _array_element (Actor|GetComponentsByClass "/Script/Engine.StaticMeshComponent")
    (Collision|SetCollisionEnabled _array_element "QueryAndPhysics")))

(fn MakeSideBuilldings
  (Development|PrintString "werwer")
  (for _index (range 0 (- (Utilities|Array|Length (Variables|Default|GetroadData)) 2))
    (Development|PrintString (Utilities|String|ToString(Vector) (* (Math|Vector|RotateVector (SplineMesh|GetStartTangent (Utilities|Array|Get(acopy) (Variables|Default|GettrackList) _index)) "0,90.000000, 0") 40)))
    (bind _returnvalue (AddComponent|AddStaticMeshComponent false (Math|Transform|MakeTransform (* (Math|Vector|RotateVector (SplineMesh|GetStartTangent (Utilities|Array|Get(acopy) (Variables|Default|GettrackList) _index)) "0,90.000000, 0") 40) "0, 0, 0" "1,1,1")))
    (Components|StaticMesh|SetStaticMesh _returnvalue "/Game/StarterContent/Geometry/Meshes/1M_Cube.1M_Cube")))