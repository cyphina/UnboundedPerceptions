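; EventBarricade is a trigger volume actor that blocks heroes from passing until a set of game conditions is met.
; When a BaseHero overlaps its box, it checks every condition through the game mode's ConditionalManager.
; On failure it moves the hero to a reset position, stops them and shows the block message as HUD dialog in that hero's name.
; On success it lets the hero through and optionally destroys itself.
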(event OnComponentBeginOverlap(Box)
  (params (OverlappedComponent :type Primitive%20Component%20Object%20Reference) (OtherActor :type Actor%20Object%20Reference) (OtherComp :type Primitive%20Component%20Object%20Reference) (OtherBodyIndex :type Integer) (bFromSweep :type Boolean) (SweepResult :type Hit%20Result%20Structure%20%28by%20ref%29))
  (if (Utilities|ClassIsChildOf (Utilities|GetClass OtherActor) "/Script/MyProject.BaseHero")
    (bind _asbase_hero (Utilities|Casting|CastToBaseHero OtherActor))
    (if (CallFunction|DoesMeetConditional?)
      ;[1 1 1] Destroy the actor if this barricade only checks once to see if conditions are fulfilled
      (if (Variables|Default|GetbIsDestroyedAfterSuccess)
        (Actor|DestroyActor))
      (else
        ;[1 1 1] If the conditionals aren't fufilled, let a popup message occur and move passing character back to preset location
        (Transformation|SetActorLocation OtherActor (Variables|Default|GetresetPosition) false false)
        (Class|Unit|Stop _asbase_hero)
        (Class|HUDManager|AddHUDDialogString (Class|UserInput|GetHUDManager (Variables|Default|GetcontrollerRef)) (CallFunction|CreateDialogLines _asbase_hero) 0 _asbase_hero)))))

(event EventBeginPlay
  (bind _asuser_input (Utilities|Casting|CastToUserInput (Game|GetPlayerController 0)))
  (Variables|Default|SetcontrollerRef _asuser_input)
  (bind _asmy_rtsgame_mode (Utilities|Casting|CastToMyRTSGameMode (Game|GetGameMode)))
  (Variables|Default|SetgameModeRef _asmy_rtsgame_mode))

(event Collision|EventActorBeginOverlap
  (params (OtherActor :type Actor%20Object%20Reference)))

(event EventTick
  (params (DeltaSeconds :type Float%20%28single-precision%29)))

(fn ConstructionScript)

(fn CreateDialogLines
  (params (heroRef :type Base%20Hero%20Object%20Reference))
  (bind _returnvalue (Class|Unit|GetGameName heroRef))
  (bind _blockmessage (Variables|Default|GetblockMessage))
  (bind _dialoglines (LocalVariables|GetdialogLines))
  (bind _returnvalue_2 (Utilities|Array|Length _blockmessage))
  (bind _returnvalue_3 (Utilities|String|ToString(Text) _returnvalue))
  (bind _returnvalue_4 (Utilities|String|StringToName _returnvalue_3))
  (for _index (range 0 (- _returnvalue_2 2))
    (Utilities|Array|Add (LocalVariables|GetdialogLines) (Utilities|Struct|MakeDialogData (Utilities|Array|MakeArray 0) (Utilities|Array|Get(acopy) _blockmessage _index) _returnvalue_4)))
  (Utilities|Array|Add _dialoglines (Utilities|Struct|MakeDialogData (Utilities|Array|MakeArray) (Utilities|Array|Get(acopy) _blockmessage (- _returnvalue_2 1)) _returnvalue_4))
  (return _dialoglines))

(fn DoesMeetConditional?
  (for _array_element (Variables|Default|Getconditions)
    (if (not (Class|ConditionalManager|GetCondition (Variables|/Script/MyProject.RTSGameMode|GetconditionalManager (Variables|Default|GetgameModeRef)) _array_element))
      (return false)))
  (return true))