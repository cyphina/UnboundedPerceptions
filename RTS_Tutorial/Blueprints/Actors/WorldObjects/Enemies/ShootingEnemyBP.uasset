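; ShootingEnemyBP is an enemy world object for the RTS that sets its initial visibility on spawn.
; After the parent BeginPlay, it checks whether its capsule overlaps any actors, intended to detect nearby allied units.
; With overlaps, it takes the player pawn as owner and hides EnemyIcon from that owner; otherwise, it hides the capsule and all its children.
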(event EventBeginPlay
  (bind _capsulecomponent (Variables|Default|GetCapsuleComponent))
  (|CallParentFunction)
  (if (> (Utilities|Array|Length (Collision|GetOverlappingActors _capsulecomponent 0 :!class /Script/Engine.PrimitiveComponent)) 0) ; Ensure we aren't initially overlapping\nany allied units
    (Actor|SetOwner (Game|Player|GetPlayerPawn 0))
    (Class|PrimitiveComponent|SetOwnerNoSee (Variables|Default|GetEnemyIcon) true)
    (else
      (Rendering|SetVisibility _capsulecomponent false true))))

(fn ConstructionScript
  (|CallParentFunction))