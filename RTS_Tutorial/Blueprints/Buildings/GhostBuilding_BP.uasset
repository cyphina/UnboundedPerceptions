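; Placement preview actor for RTS build mode, showing a ghost mesh and direction arrow for the chosen building.
; ConstructBuilding briefly spawns a building to read its mesh and work hours, then activates the ghost.
; While active, gated Tick grid-snaps it to the cursor, checks overlaps, then uses corner and centre traces for slope and a box trace for height.
; Invalid spots get an error material; GetConstructionStruct packages the placement.
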(event Custom|OnSpawn
  (params (BuildingClass :type Building%20Master%20BP%20Class%20Reference) (DisplayMesh :type Static%20Mesh%20Object%20Reference) (workHours :type Float%20%28single-precision%29))
  (bind _arrow (Variables|Default|GetArrow))
  ;[1 1 1] On Spawn
  (if (not (Variables|Default|GetisActive))
    (Variables|Default|SetBuildingClass BuildingClass)
    (Variables|Default|SetdisplayMesh DisplayMesh)
    (Variables|Default|SetworkHoursRequired workHours)
    (Variables|Default|SetisActive true)
    (Variables|/Game/RTS_Tutorial/Blueprints/GameBP/CameraPawnController.CameraPawnController_C|SetbuildModeActive (Variables|Default|GetControllerRef) true)
    (Components|StaticMesh|SetStaticMesh (Variables|Default|GetGhostBuilding_Mesh) (Variables|Default|GetdisplayMesh))
    (CallFunction|OpenTickGate)
    (bind _output_get (Variables|Default|Setextent (.BoxExtent (Collision|GetComponentBounds (Variables|Default|GetGhostBuilding_Mesh)))))
    (Transformation|SetRelativeLocation _arrow (Math|Vector|MakeVector (.x _output_get) 0.0 0.0) false false)
    (Development|SetHiddeninGame _arrow false false)
    (CallFunction|SetBuildingCollisionBox (Variables|Default|GetCollision) (Variables|Default|GetGhostBuilding_Mesh))))

(event Custom|KillGhost
  ;[1 1 1] Kill Ghost
  (Variables|Default|SetBuildingClass 0)
  (Variables|Default|SetConstructionProxy 0)
  (CallFunction|CloseTickGate)
  (Variables|Default|SetdisplayMesh 0)
  (Variables|Default|SetisActive false)
  (Variables|/Game/RTS_Tutorial/Blueprints/GameBP/CameraPawnController.CameraPawnController_C|SetbuildModeActive (Variables|Default|GetControllerRef) false)
  (Components|StaticMesh|SetStaticMesh (Variables|Default|GetGhostBuilding_Mesh) (Variables|Default|GetdisplayMesh))
  (Transformation|SetActorRotation "0, 0, 0")
  (Development|SetHiddeninGame (Variables|Default|GetArrow) true false))

(event Custom|OpenTickGate
  ;[1 1 1] Tick
  (Utilities|FlowControl|Gate true) ; enters at Open
)

(event Custom|CloseTickGate
  ;[1 1 1] Tick
  (Utilities|FlowControl|Gate true) ; enters at Close
)

(event Custom|SetMaterial
  (bind _ghostbuilding_mesh (Variables|Default|GetGhostBuilding_Mesh))
  ;[1 1 1] Overlapping Material
  (if (Variables|Default|GetisOverlapping)
    (Rendering|Material|SetMaterial _ghostbuilding_mesh 0 "/Game/RTS_Tutorial/Materials/EffectMats/GhostError_M_Inst.GhostError_M_Inst")
    (else
      (Rendering|Material|SetMaterial _ghostbuilding_mesh 0 "/Game/RTS_Tutorial/Materials/EffectMats/Ghost_M_Inst.Ghost_M_Inst"))))

(event EventConstructBuilding
  (params (MainBuilding :type Building%20Master%20BP%20Class%20Reference))
  ;[1 1 1] Building Construction
  (bind _returnvalue (Game|SpawnActorfromClass "/Game/RTS_Tutorial/Blueprints/Buildings/BuildingMasterBP.BuildingMasterBP_C" (Math|Transform|MakeTransform "0, 0, 0") "Undefined" 0 0 0))
  (Utilities|FlowControl|Sequence
    (:then_0
      (bind _asbuilding_master_bp (Utilities|Casting|CastToBuildingMasterBPClass MainBuilding))
      (CallFunction|KillGhost)
      (CallFunction|OnSpawn _asbuilding_master_bp (Variables|/Game/RTS_Tutorial/Blueprints/Buildings/BuildingMasterBP.BuildingMasterBP_C|GetDisplayMesh _returnvalue) (Variables|/Game/RTS_Tutorial/Blueprints/Buildings/BuildingMasterBP.BuildingMasterBP_C|GetconstructionTime _returnvalue)))
    (:then_1
      (Actor|DestroyActor _returnvalue))))

(event EventTick
  (params (DeltaSeconds :type Float%20%28single-precision%29))
  ;[1 1 1] Tick
  (Utilities|FlowControl|Gate true
    (:Exit
      (Transformation|SetActorLocation self (CallFunction|SetGridSnapVector) false false)
      (if (CallFunction|CheckOverlap)
        (Variables|Default|SetisOverlapping true)
        (CallFunction|SetMaterial)
        (else
          (bind _badlocation (CallFunction|CalculateSlope))
          (Variables|Default|SetisOverlapping _badlocation)
          (CallFunction|SetMaterial))))))

(fn ConstructionScript)

(fn SetGridSnapVector
  (bind _cursorworldposition (Variables|Default|GetcursorWorldPosition))
  (bind _gridsize (Variables|Default|GetgridSize))
  (return (Math|Vector|MakeVector (CallFunction|GridSnap (.x _cursorworldposition) _gridsize) (CallFunction|GridSnap (.y _cursorworldposition) _gridsize) (CallFunction|GridSnap (.z _cursorworldposition) _gridsize))))

(fn SetCursorWorldPosition
  (params (CursorLocation :type Vector))
  (Variables|Default|SetcursorWorldPosition CursorLocation)
  (return))

(fn GetConstructionStruct
  (return (Utilities|Struct|MakeConstruction_Struct (Variables|Default|GetBuildingClass) (Math|Transform|MakeTransform (Transformation|GetActorLocation) (Transformation|GetActorRotation)) (Variables|Default|GetdisplayMesh) (Variables|Default|GetworkHoursRequired))))

(fn CheckOverlap
  (return (> (Utilities|Array|Length (Collision|GetOverlappingActors "/Script/Engine.Actor" :!class /Script/Engine.Actor)) 0)))

(fn CalculateSlope
  (bind (_actorlocation _forwardvector _rightvector) (CallFunction|GetVectors))
  (bind (_actorlocation_2 _forwardvector_2 _rightvector_2) (CallFunction|GetVectors))
  (bind (_actorlocation_3 _forwardvector_3 _rightvector_3) (CallFunction|GetVectors))
  (bind (_actorlocation_4 _forwardvector_4 _rightvector_4) (CallFunction|GetVectors))
  (bind _actorlocation_5 (CallFunction|GetVectors))
  (bind _actorlocation_6 (CallFunction|GetVectors))
  (bind _extent (Variables|Default|Getextent))
  (bind _maxdifferences (LocalVariables|GetmaxDifferences))
  (bind _differences (LocalVariables|Getdifferences))
  (bind (_indexofminvalue _minvalue) (Math|Float|MinOfFloatArray _differences))
  (bind (_indexofmaxvalue _maxvalue) (Math|Float|MaxOfFloatArray _differences))
  (Utilities|FlowControl|Sequence
    (:then_0
      (Utilities|FlowControl|Sequence
        (:then_0
          ;[1 0.6033 0.8012] Get corners of object.  Then trace line directly below them and see how far the landscape is from that corner
          (bind _difference (CallFunction|SlopeTrace (+ _actorlocation (* (+ _forwardvector _rightvector) (Variables|Default|Getextent)))))
          (Utilities|Array|Add (LocalVariables|Getdifferences) _difference))
        (:then_1
          (bind _difference_2 (CallFunction|SlopeTrace (+ _actorlocation_2 (* (+ (* _forwardvector_2 -1.0) _rightvector_2) (Variables|Default|Getextent)))))
          (Utilities|Array|Add (LocalVariables|Getdifferences) _difference_2))
        (:then_2
          (bind _difference_3 (CallFunction|SlopeTrace (+ _actorlocation_3 (* (+ _forwardvector_3 (* _rightvector_3 -1.0)) (Variables|Default|Getextent)))))
          (Utilities|Array|Add (LocalVariables|Getdifferences) _difference_3))
        (:then_3
          (bind _difference_4 (CallFunction|SlopeTrace (+ _actorlocation_4 (* (+ (* _forwardvector_4 -1.0) (* _rightvector_4 -1.0)) (Variables|Default|Getextent)))))
          (Utilities|Array|Add (LocalVariables|Getdifferences) _difference_4))
        (:then_4
          (bind _difference_5 (CallFunction|SlopeTrace (.actorLocation (CallFunction|GetVectors))))
          (Utilities|Array|Add (LocalVariables|Getdifferences) _difference_5))))
    (:then_1
      (if (and (> _indexofminvalue -1) (> _indexofmaxvalue -1))
        (bind (_outhit _returnvalue) (Class|KismetSystemLibrary|BoxTraceSingleforObjects (+ _actorlocation_5 "0,0.000000,1000.000000") (- _actorlocation_5 "0, 0,1000.000000") (Math|Vector|MakeVector (.x _extent) (.y _extent) 1.0) "0, 0, 0" (Utilities|Array|MakeArray "ObjectTypeQuery7") false 0 "ForOneFrame" true))
        (if _returnvalue
          (Transformation|SetActorLocation (Math|Vector|MakeVector (.x _actorlocation_6) (.y _actorlocation_6) (.z (.ImpactPoint (Collision|BreakHitResult _outhit)))) false false))))
    (:then_2
      (return (or (> (Math|Float|Absolute(Float) _minvalue) _maxdifferences) (> (Math|Float|Absolute(Float) _maxvalue) _maxdifferences))))))

(fn GetVectors
  (bind _returnvalue (Transformation|GetActorRotation))
  (return (Transformation|GetActorLocation) (Math|Vector|GetForwardVector _returnvalue) (Math|Vector|GetRightVector _returnvalue)))

(fn SlopeTrace
  (params (TraceLocation :type Vector))
  (bind _outhit (Collision|LineTraceByChannel (+ TraceLocation "0, 0,1000.000000") (- TraceLocation "0, 0,1000.000000") "TraceTypeQuery3" false 0 "None"))
  (return (- (.z (Transformation|GetActorLocation)) (.z (.Location (Collision|BreakHitResult _outhit))))))

(fn GetIsOverlapping
  (return (Variables|Default|GetisOverlapping)))

(fn SetCalendar
  (params (Date :type Array%20of%20Integers))
  (return false))

(fn SetClock
  (params (Time :type Array%20of%20Integers))
  (return false))