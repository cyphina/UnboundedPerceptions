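; Base building Blueprint for an RTS, showing a building HUD when the building is selected.
; The construction script applies the display mesh and passes it to helper functions that set the entrance and collision box.
; On BeginPlay it binds to the camera pawn controller's HUD request and creates its Building_HUD widget.
; When a display request names this actor, it adds that widget to the viewport.
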(event Custom|DisplayHUD
  (params (actor :type Actor%20Object%20Reference))
  ;[1 1 1] Is this actor selecting me?
  (if (== actor self)
    (UserInterface|Viewport|AddtoViewport (Variables|Default|GetbuildingHUD) 0)))

(event EventBeginPlay
  (bind _ascamera_pawn_controller (Utilities|Casting|CastToCameraPawnController (Game|GetPlayerController 0)))
  (bind _output_get (Variables|References|SetControllerRef _ascamera_pawn_controller))
  (EventDispatchers|BindEventtoHUDRequest _output_get (EventDispatchers|CreateEvent :!event Custom|DisplayHUD))
  (bind _returnvalue (UserInterface|CreateWidget "/Game/RTS_Tutorial/HUDs/Building_HUD.Building_HUD_C"))
  (Variables|Default|SetbuildingHUD _returnvalue))

(fn ConstructionScript
  (Components|StaticMesh|SetStaticMesh (Variables|Default|GetStaticMesh) (Variables|Default|GetDisplayMesh))
  (CallFunction|SetBuildingEntrance (Variables|Default|GetEntrance) (Variables|Default|GetStaticMesh))
  (CallFunction|SetBuildingCollisionBox (Variables|Default|GetCollision) (Variables|Default|GetStaticMesh)))