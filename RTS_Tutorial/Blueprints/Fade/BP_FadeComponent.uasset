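; Actor component that fades its owning StaticMeshActor out and back in when ToggleHideMesh is called.
; BeginPlay caches the mesh's slot 0 material, which must be a base Material, and creates a dynamic instance of FadeMaterial.
; Hiding swaps in that instance, while Tick drives its Fade parameter through a curve at FadeRate.
; The original material returns once the mesh is fully visible.
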(event EventBeginPlay
  (bind _asstatic_mesh_actor (Utilities|Casting|CastToStaticMeshActor (Components|GetOwner)))
  (bind _output_get (Variables|Default|SetparentMesh _asstatic_mesh_actor))
  (bind _asmaterial (Utilities|Casting|CastToMaterial (Rendering|Material|GetMaterial (Variables|/Script/Engine.StaticMeshActor|GetStaticMeshComponent _output_get) 0)))
  (Variables|Default|SetBaseMaterial _asmaterial)
  (bind _returnvalue (Rendering|Material|CreateDynamicMaterialInstance (Variables|Default|GetFadeMaterial) :!class /Script/Engine.KismetMaterialLibrary))
  (Variables|Default|SetFadeMaterialMID _returnvalue))

(event EventTick
  (params (DeltaSeconds :type Float%20%28single-precision%29))
  (Variables|Default|SetdeltaTime DeltaSeconds)
  (if (Variables|Default|Gethidden)
    (Variables|Default|SetcurrentFade (Math|Float|Clamp(Float) (- (Variables|Default|GetcurrentFade) (* (Variables|Default|GetdeltaTime) (Variables|Default|GetFadeRate)))))
    (else
      (Variables|Default|SetcurrentFade (Math|Float|Clamp(Float) (+ (Variables|Default|GetcurrentFade) (* (Variables|Default|GetdeltaTime) (Variables|Default|GetFadeRate)))))))
  (Rendering|Material|SetScalarParameterValue (Variables|Default|GetFadeMaterialMID) "Fade" (Math|Curves|GetFloatValue (Variables|Default|GetfadeCurve) (Variables|Default|GetcurrentFade)) :!class /Script/Engine.MaterialInstanceDynamic)
  (if (and (== (Variables|Default|GetcurrentFade) 1.0) (not (Variables|Default|Gethidden)))
    (Rendering|Material|SetMaterial (Variables|/Script/Engine.StaticMeshActor|GetStaticMeshComponent (Variables|Default|GetparentMesh)) 0 (Variables|Default|GetBaseMaterial))))

(fn ToggleHideMesh
  (params (hidden :type Boolean))
  (if (Math|Boolean|NotEqual(Boolean) hidden (Variables|Default|Gethidden))
    (bind _output_get (Variables|Default|Sethidden hidden))
    (if _output_get
      (Rendering|Material|SetMaterial (Variables|/Script/Engine.StaticMeshActor|GetStaticMeshComponent (Variables|Default|GetparentMesh)) 0 (Variables|Default|GetFadeMaterialMID)))))