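; Camera pawn with a spring arm, whose length sets the camera zoom.
; On BeginPlay it disables its input from the first player controller, snaps to the world origin with a fixed rotation and makes a hardware cursor call with no cursor name.
; SetCameraArmLength treats its NewLength argument as a delta, adding it to the current arm length and clamping between a fixed minimum and MaxArmDistance.
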(event EventBeginPlay
  (Input|DisableInput (Game|GetPlayerController 0))
  (Transformation|SetActorLocation "0, 0, 0" false false)
  (Transformation|SetActorRotation "0,-180.000000, 0")
  (Class|WidgetBlueprintLibrary|SetHardwareCursor "None" "None"))

(event Collision|EventActorBeginOverlap
  (params (OtherActor :type Actor%20Object%20Reference)))

(event EventSetCameraArmLength
  (params (newLength :type Float%20%28single-precision%29))
  (bind _springarm (Variables|Default|GetSpringArm))
  (Variables|/Script/Engine.SpringArmComponent|SetTargetArmLength _springarm (Math|Float|Clamp(Float) (+ newLength (Variables|/Script/Engine.SpringArmComponent|GetTargetArmLength _springarm)) 2.5e+02 (Variables|Default|GetmaxArmDistance))))

(fn ConstructionScript)