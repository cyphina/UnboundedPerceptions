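; Functional test that verifies a spawned Ally registers itself in the base player's Allies list.
; IsReady waits for a valid player pawn with a CameraPawnController and caches that controller.
; StartTest records the party size, spawns an Ally, and succeeds only if the list has grown by exactly one.
; The spawned Ally is destroyed before the test reports success or failure.
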(event EventPrepareTest)

(event EventStartTest
  (bind _cpcref (Variables|Default|GetcpcRef))
  (bind _returnvalue (Class|UserInput|GetBasePlayer _cpcref))
  (bind _allies (Variables|/Script/MyProject.BasePlayer|Getallies _returnvalue))
  (bind _returnvalue_2 (Utilities|Array|Length _allies))
  (bind _output_get (Variables|Default|SetpartySize _returnvalue_2))
  (bind _returnvalue_3 (Game|SpawnActorfromClass :Class "/Script/MyProject.Ally" :CollisionHandlingOverride "Undefined" :Instigator 0))
  (Utilities|IsValid _returnvalue_3
    (:Is%20Valid
      (if (== _returnvalue_2 (+ _output_get 1))
        (Actor|DestroyActor _returnvalue_3)
        (Class|FunctionalTest|FinishTest "Succeeded" "Ally Spawned Successfully")
        (else
          (Actor|DestroyActor _returnvalue_3 :!label _label)
          (Class|FunctionalTest|FinishTest "Failed" "Test Failed"))))
    (:Is%20Not%20Valid
      (goto _label))))

(event EventTick
  (params (DeltaSeconds :type Float%20%28single-precision%29)))

(fn ConstructionScript)

(fn IsReady
  (bind _returnvalue (Game|Player|GetPlayerPawn 0))
  (if (Utilities|IsValid _returnvalue)
    (bind _ascamera_pawn_controller (Utilities|Casting|CastToCameraPawnController (Pawn|GetController _returnvalue)))
    (Variables|Default|SetcpcRef _ascamera_pawn_controller)
    (return (Utilities|IsValid _ascamera_pawn_controller))))