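; Construction worker NPC for the RTS, with a randomized identity, a selection HUD and an AI busy flag.
; Construction picks a random sex to tint a dynamic body material and fill the name profile, though only male names are randomized.
; BeginPlay binds controller HUD requests, showing its widget when selected, and game-speed updates that scale walk speed.
; SetIsBusy writes the busy state to the AI blackboard.
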(event Custom|DisplayHUD
  (params (actor :type Actor%20Object%20Reference))
  ;[1 1 1] Is this actor selecting me?
  (if (== actor self)
    (UserInterface|Viewport|AddtoViewport (Variables|Default|GetproxyHUD) 0)))

(event Custom|UpdateGameSpeed
  (params (SpeedMultiplier :type Float%20%28single-precision%29))
  (Variables|/Script/Engine.CharacterMovementComponent|SetMaxWalkSpeed (Variables|Character|GetCharacterMovement) (* (Variables|Default|GetbaseWalkSpeed) (Variables|/Script/MyProject.RTSGameState|GetspeedModifier (Variables|Default|GetgameStateRef)))))

(event EventBeginPlay
  (Utilities|Casting|CastToConstructionNPCController (AI|GetAIController self))
  (Variables|Default|SetAIControllerRef 0)
  (bind _ascamera_pawn_controller (Utilities|Casting|CastToCameraPawnController (Game|GetPlayerController 0)))
  (bind _output_get (Variables|Default|SetcameraPawnController _ascamera_pawn_controller))
  (EventDispatchers|BindEventtoHUDRequest _output_get (EventDispatchers|CreateEvent :!event Custom|DisplayHUD))
  (bind _returnvalue (UserInterface|CreateWidget "/Game/RTS_Tutorial/HUDs/StatUI/NPC_HUD.NPC_HUD_C"))
  (Variables|Default|SetproxyHUD _returnvalue)
  (EventDispatchers|BindEventtoUpdateGameSpeedDelegate (Variables|Default|GetgameStateRef) (EventDispatchers|CreateEvent :!event Custom|UpdateGameSpeed))
  (Variables|/Script/Engine.CharacterMovementComponent|SetMaxWalkSpeed (Variables|Character|GetCharacterMovement) (* (Variables|Default|GetbaseWalkSpeed) (Variables|/Script/MyProject.RTSGameState|GetspeedModifier (Variables|Default|GetgameStateRef)))))

(event Collision|EventActorBeginOverlap
  (params (OtherActor :type Actor%20Object%20Reference)))

(event EventTick
  (params (DeltaSeconds :type Float%20%28single-precision%29)))

(fn ConstructionScript
  (CallFunction|RandomNPCFeatures))

(fn RandomNPCFeatures
  (bind _returnvalue (Rendering|Material|CreateDynamicMaterialInstance (Variables|Character|GetMesh) 0 0 "None" :!class /Script/Engine.PrimitiveComponent))
  (LocalVariables|SetmaterialInstance _returnvalue)
  (if (Utilities|Enum|Equal(Enum) (Utilities|Enum|LiteralenumSex (Utilities|Enum|ByteToEnumSex (Math|Conversions|ToByte(Integer) (Math|Random|RandomIntegerinRange 0 1)))) "NewEnumerator0")
    (Rendering|Material|SetVectorParameterValue (LocalVariables|GetmaterialInstance) "BodyColor" (LocalVariables|GetmaleColor) :!class /Script/Engine.MaterialInstanceDynamic)
    (bind _name (CallFunction|GetRandomName "NewEnumerator0"))
    (Variables|Default|SetmyProfile (Utilities|Struct|MakeNPCProfile_Struct _name "NewEnumerator0"))
    (else
      (Rendering|Material|SetVectorParameterValue (LocalVariables|GetmaterialInstance) "BodyColor" (LocalVariables|GetfemaleColor) :!class /Script/Engine.MaterialInstanceDynamic)
      (bind _name_2 (CallFunction|GetRandomName "NewEnumerator1"))
      (Variables|Default|SetmyProfile (Utilities|Struct|MakeNPCProfile_Struct _name_2 "NewEnumerator0")))))

(fn GetRandomName
  (params (gender :type Sex%20Enum :default "NewEnumerator0"))
  (if (Utilities|Enum|Equal(Enum) gender "NewEnumerator0")
    (return (Utilities|String|EnumtoString (Utilities|Enum|LiteralenumNPCNameMale_ENUM (Utilities|Enum|ByteToEnumNPCNameMale_ENUM (Math|Conversions|ToByte(Integer) (Math|Random|RandomIntegerinRange 0 (- (|GetNumEnumEntries) 1)))))))
    (else
      (return (Utilities|String|EnumtoString (Utilities|Enum|ByteToEnumNPCNameMale_ENUM))))))

(fn SetIsBusy
  (params (isBusy :type Boolean))
  (AI|Components|Blackboard|SetValueasBool (AI|GetBlackboard (Variables|Default|GetAIControllerRef)) (LocalVariables|GetbusyName) isBusy)
  (return))