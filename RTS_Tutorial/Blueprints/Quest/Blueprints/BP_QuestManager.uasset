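; Quest manager Blueprint for an RTS, containing only disconnected logic that never runs and an empty construction script.
; The dormant graph replaces the current goal marker with a radius-circle BP_GoalActor at the selected quest's selected subgoal location, then calls ParentOnSwitchSubGoal.
; Subgoals whose location matches the invalid-vector sentinel instead clear the marker reference and hide the quest list's distance indicator.
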(fn ConstructionScript)