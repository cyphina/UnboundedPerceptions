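; Actor component that fades its owning static mesh actor out and back in, registering itself in the game state's FadeComponents.
; ToggleHideMesh sets the hidden flag and, when hiding, puts a dynamic fade material on all slots.
; While recently rendered, Tick drives that material's Fade parameter through a curve.
; Gates switch a custom collision channel to Ignore once fully faded, or restore Block and slot 0's base material once visible.
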(event EventBeginPlay
  (bind _asstatic_mesh_actor (Utilities|Casting|CastToStaticMeshActor (Components|GetOwner)))
  (bind _output_get (Variables|Default|SetparentMesh _asstatic_mesh_actor))
  (bind _asmaterial_instance (Utilities|Casting|CastToMaterialInstance (Rendering|Material|GetMaterial (Variables|/Script/Engine.StaticMeshActor|GetStaticMeshComponent _output_get) 0))
    (:then
      (Variables|Default|SetBaseMaterial _asmaterial_instance))
    (:CastFailed
      (bind _returnvalue (Rendering|Material|CreateDynamicMaterialInstance (Rendering|Material|GetMaterial (Variables|/Script/Engine.StaticMeshActor|GetStaticMeshComponent _output_get) 0) "None" :!class /Script/Engine.KismetMaterialLibrary))
      (Variables|Default|SetBaseMaterial _returnvalue)))
  (bind _returnvalue_2 (Rendering|Material|CreateDynamicMaterialInstance (Variables|Default|GetFadeMaterial) "None" :!class /Script/Engine.KismetMaterialLibrary))
  (Variables|Default|SetFadeMaterialMID _returnvalue_2)
  (Collision|SetCollisionResponsetoChannel (Variables|/Script/Engine.StaticMeshActor|GetStaticMeshComponent (Variables|Default|GetparentMesh)) "ECC_GameTraceChannel12" "ECR_Overlap")
  (bind _asmy_game_state (Utilities|Casting|CastToMyGameState (Game|GetGameState)))
  (Utilities|Array|Add (Variables|/Game/RTS_Tutorial/Blueprints/GameBP/MyGameState.MyGameState_C|GetfadeComponents _asmy_game_state) self))

(event EventTick
  (params (DeltaSeconds :type Float%20%28single-precision%29))
  (bind _parentmesh (Variables|Default|GetparentMesh))
  (bind _staticmeshcomponent (Variables|/Script/Engine.StaticMeshActor|GetStaticMeshComponent _parentmesh))
  (if (Class|Actor|WasRecentlyRendered (Variables|Default|GetparentMesh) 0.1)
    (Variables|Default|SetdeltaTime DeltaSeconds)
    (if (Variables|Default|Gethidden)
      ;[1 1 1] Fade Away...
      (Variables|Default|SetcurrentFade (Math|Float|Clamp(Float) (- (Variables|Default|GetcurrentFade) (* (Variables|Default|GetdeltaTime) (Variables|Default|GetFadeRate)))))
      (else
        ;[1 1 1] Fade In...
        (Variables|Default|SetcurrentFade (Math|Float|Clamp(Float) (+ (Variables|Default|GetcurrentFade) (* (Variables|Default|GetdeltaTime) (Variables|Default|GetFadeRate)))))))
    (Rendering|Material|SetScalarParameterValue (Variables|Default|GetFadeMaterialMID) "Fade" (Math|Curves|GetFloatValue (Variables|Default|GetfadeCurve) (Variables|Default|GetcurrentFade)) :!class /Script/Engine.MaterialInstanceDynamic)
    (if (not (Variables|Default|Gethidden))
      (if (== (Variables|Default|GetcurrentFade) 1.0)
        (Utilities|FlowControl|Gate false :!label _label
          (:Exit
            (Rendering|Material|SetMaterial _staticmeshcomponent 0 (Variables|Default|GetBaseMaterial))
            (Collision|SetCollisionResponsetoChannel _staticmeshcomponent "ECC_GameTraceChannel1" "ECR_Block")
            (goto _label Close)))
        (else
          (goto _label Open)))
      (elif (== (Variables|Default|GetcurrentFade) 0.0)
        (Utilities|FlowControl|Gate false :!label _label_2
          (:Exit
            (Collision|SetCollisionResponsetoChannel _staticmeshcomponent "ECC_GameTraceChannel1" "ECR_Ignore")
            (goto _label_2 Close)))
        (else
          (goto _label_2 Open))))))

(fn ToggleHideMesh
  (params (hidden :type Boolean))
  (bind _parentmesh (Variables|Default|GetparentMesh))
  (bind _staticmeshcomponent (Variables|/Script/Engine.StaticMeshActor|GetStaticMeshComponent _parentmesh))
  (if (Math|Boolean|NotEqual(Boolean) hidden (Variables|Default|Gethidden))
    (bind _output_get (Variables|Default|Sethidden hidden))
    (if _output_get
      (for _index (range 0 (Rendering|Material|GetNumMaterials _staticmeshcomponent))
        (Rendering|Material|SetMaterial _staticmeshcomponent _index (Variables|Default|GetFadeMaterialMID))))))

(fn StopFade
  (bind _parentmesh (Variables|Default|GetparentMesh))
  (bind _staticmeshcomponent (Variables|/Script/Engine.StaticMeshActor|GetStaticMeshComponent _parentmesh))
  (Rendering|Material|SetScalarParameterValue (Variables|Default|GetFadeMaterialMID) "Fade" 0.0 :!class /Script/Engine.MaterialInstanceDynamic)
  (Variables|Default|SetcurrentFade 0.0)
  (Rendering|Material|SetMaterial _staticmeshcomponent 0 (Variables|Default|GetBaseMaterial))
  (Collision|SetCollisionResponsetoChannel _staticmeshcomponent "ECC_GameTraceChannel1" "ECR_Block")
  (Variables|Default|Sethidden false))