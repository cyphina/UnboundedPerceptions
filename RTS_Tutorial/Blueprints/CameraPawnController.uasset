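; RTS player controller that drives the camera pawn, hero selection and orders, and building placement.
; BeginPlay spawns a construction manager and ghost building and creates the main HUD.
; Input handles zoom-scaled movement, edge scrolling, panning, click or box selection, right-click moves, and rotating and queueing ghost buildings.
; A looping timer uses hero overlap hits to toggle fade components on static meshes that get hidden.
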(event Custom|DrawMouseSelection
  (bind (_locationx _locationy) (Game|Player|GetMousePosition))
  (bind _startmouseposition (Variables|Mouse|GetstartMousePosition))
  (bind _hud (Variables|References|GetHud))
  (bind (_x _y) (Math|Vector2D|BreakVector2D _startmouseposition))
  ;[1 1 1] Selection Box
  (Variables|Mouse|SetendMousePosition (Math|Vector2D|MakeVector2D _locationx _locationy))
  (if (CallFunction|IsRect)
    (HUD|DrawRect _hud "(R=0.785000,G=0.424373,B=0.767152,A=0.436000)" _x _y (.X (Math|Vector2D|BreakVector2D (- (Variables|Mouse|GetendMousePosition) _startmouseposition))) (.Y (Math|Vector2D|BreakVector2D (- (Variables|Mouse|GetendMousePosition) _startmouseposition))))
    (for _array_element (Class|HUD|GetActorsinSelectionRectangle _hud "/Script/MyProject.BaseHero" _startmouseposition (Variables|Mouse|GetendMousePosition) false false)
      (if (.bSuccess (Utilities|Casting|CastToBaseHero _array_element))
        (Class|Unit|SetSelected (.AsBase%20Hero (Utilities|Casting|CastToBaseHero _array_element)) true)))))

(event Custom|startClick
  (bind _hitobject (CallFunction|GetHitObject))
  (bind _hitobject_2 (CallFunction|GetHitObject))
  (bind (_asbase_hero _bsuccess) (Utilities|Casting|CastToBaseHero _hitobject_2))
  (bind (_asbase_hero_2 _bsuccess_2) (Utilities|Casting|CastToBaseHero _hitobject))
  ;[1 0.4034 0.5237] Left Click Selection
  (|SetStartClick)
  (if (Game|Player|IsInputKeyDown "LeftShift")
    (Utilities|HeroCheck
      (:then
        (if _bsuccess_2
          (if (Class|Unit|GetSelected _asbase_hero_2)
            (Class|Unit|SetSelected _asbase_hero_2 false)
            (else
              (Class|Unit|SetSelected _asbase_hero_2 true))))))
    (else
      (Utilities|FlowControl|Sequence
        (:then_0
          (bind _array_element (Utilities|HeroLoop)
            (:LoopBody
              (Class|Unit|SetSelected _array_element false))))
        (:then_1
          (Utilities|HeroCheck
            (:then
              (if _bsuccess
                (Class|Unit|SetSelected _asbase_hero true)))
            (:else
              (Default|CallHUDRequest _hitobject_2))))))))

(event Custom|whileClicked
  ;[1 1 1] Update Selection Rect - Updates the end of the rectangle
)

(event EventBeginPlay
  (bind _returnvalue (Math|Transform|MakeTransform "0, 0, 0"))
  (bind _self self)
  ;[0 0 0] Begin Play
  (Utilities|FlowControl|Sequence
    (:then_0
      (Utilities|ReferenceCasts))
    (:then_1
      (bind _returnvalue_2 (Game|SpawnActorfromClass "/Game/RTS_Tutorial/Blueprints/Construction/ConstructionManager_BP.ConstructionManager_BP_C" _returnvalue "AlwaysSpawn" 0 0))
      (Variables|References|SetConstructionManagerRef _returnvalue_2))
    (:then_2
      (bind _returnvalue_3 (Game|SpawnActorfromClass "/Game/RTS_Tutorial/Blueprints/Buildings/GhostBuilding_BP.GhostBuilding_BP_C" _returnvalue "AlwaysSpawn" 0 _self 0))
      (Variables|References|SetGhostBuildingRef _returnvalue_3))
    (:then_3
      (bind _outactors (Actor|GetAllActorsOfClass "/Script/MyProject.BasePlayer"))
      (Variables|References|SetbasePlayer (Utilities|Array|Get(acopy) _outactors)))
    (:then_4
      (Input|SetInputModeGameandUI _self 0 "LockOnCapture" false)
      (Utilities|CreateHuds)
      (UserInterface|Viewport|AddtoViewport (Variables|References|GetMainHudRef) 0))
    (:then_5
      (Utilities|Time|SetTimerbyFunctionName 0 "UpdateFadeActors" 0.1 true))))

(event EventTick
  (params (DeltaSeconds :type Float%20%28single-precision%29))
  ;[1 1 1] Follow Cursor
  (Utilities|FlowControl|Sequence
    (:then_0
      (if (Variables|Building|GetbuildModeActive)
        (|SetCursorWorldPosition)))
    (:then_1
      ;[1 1 1] Update Selection Rect - Updates the end of the rectangle
      (if (> (Class|PlayerController|GetInputKeyTimeDown "LeftMouseButton") 0.05)
        (CallFunction|WhileClicked)))))

(event Input|ActionEvents|InputActionPan
  (params (Key :type Key%20Structure :default "AnyKey"))
  (bind _camerapawnref (Variables|References|GetCameraPawnRef))
  (bind _returnvalue (Transformation|GetActorRotation _camerapawnref))
  (bind (_roll _pitch _yaw) (Math|Rotator|BreakRotator _returnvalue))
  ;[0.5198 0.8997 1] Camera Movement
  ;;[1 1 1] Pan Y
  (:Pressed
    (Variables|Camera|SetdisableCamNav true)
    (Utilities|FlowControl|Gate true) ; enters at Open
  )
  (:Released
    (Variables|Camera|SetdisableCamNav false)
    (Utilities|FlowControl|Gate true) ; enters at Close
  ))

(event Input|ActionEvents|InputActionZoomOut
  (params (Key :type Key%20Structure :default "AnyKey"))
  (bind _camerapawnref (Variables|References|GetCameraPawnRef))
  (bind _springarm (Variables|/Game/RTS_Tutorial/Blueprints/CameraPawn.CameraPawn_C|GetSpringArm _camerapawnref))
  ;[0.5198 0.8997 1] Camera Movement
  ;;[1 1 1] Zoom In/Out
  (:Pressed
    (Variables|/Script/Engine.SpringArmComponent|SetTargetArmLength _springarm (Math|Float|Clamp(Float) (+ (Variables|Camera|GetzoomSensitivity) (Variables|/Script/Engine.SpringArmComponent|GetTargetArmLength _springarm)) 5e+02 (Variables|Camera|GetmaxArmDistance)))))

(event Input|ActionEvents|InputActionPan
  (params (Key :type Key%20Structure :default "AnyKey"))
  (bind _camerapawnref (Variables|References|GetCameraPawnRef))
  (bind _returnvalue (Transformation|GetActorRotation _camerapawnref))
  (bind (_roll _pitch _yaw) (Math|Rotator|BreakRotator _returnvalue))
  ;[0.5198 0.8997 1] Camera Movement
  ;;[1 1 1] Pan X
  (:Pressed
    (Variables|Camera|SetdisableCamNav true)
    (Utilities|FlowControl|Gate true) ; enters at Open
  )
  (:Released
    (Variables|Camera|SetdisableCamNav false)
    (Utilities|FlowControl|Gate true) ; enters at Close
  ))

(event Input|ActionEvents|InputActionZoomReset
  (params (Key :type Key%20Structure :default "AnyKey"))
  ;[0.5198 0.8997 1] Camera Movement
  ;;[1 1 1] Zoom Reset
  (:Pressed
    (Variables|/Script/Engine.SpringArmComponent|SetTargetArmLength (Variables|/Game/RTS_Tutorial/Blueprints/CameraPawn.CameraPawn_C|GetSpringArm (Variables|References|GetCameraPawnRef)) 1.5e+03)))

(event Input|ActionEvents|InputActionRotateBuildingLeft
  (params (Key :type Key%20Structure :default "AnyKey"))
  (bind _ghostbuildingref (Variables|References|GetGhostBuildingRef))
  (bind _returnvalue (Transformation|GetActorRotation _ghostbuildingref))
  (bind (_roll _pitch _yaw) (Math|Rotator|BreakRotator _returnvalue))
  ;[1 1 1] Building Rotation
  (:Pressed
    (if (and (Variables|Building|GetbuildModeActive) (Utilities|IsValid _ghostbuildingref))
      (Transformation|SetActorRotation _ghostbuildingref (Math|Rotator|MakeRotator _roll _pitch (- _yaw (Variables|Default|GetbuildRotationRate)))))))

(event Input|ActionEvents|InputActionRotateBuildingRight
  (params (Key :type Key%20Structure :default "AnyKey"))
  (bind _ghostbuildingref (Variables|References|GetGhostBuildingRef))
  (bind _returnvalue (Transformation|GetActorRotation _ghostbuildingref))
  (bind (_roll _pitch _yaw) (Math|Rotator|BreakRotator _returnvalue))
  ;[1 1 1] Building Rotation
  (:Pressed
    (if (and (Variables|Building|GetbuildModeActive) (Utilities|IsValid _ghostbuildingref))
      (Transformation|SetActorRotation _ghostbuildingref (Math|Rotator|MakeRotator _roll _pitch (+ _yaw (Variables|Default|GetbuildRotationRate)))))))

(event Input|ActionEvents|InputActionPanReset
  (params (Key :type Key%20Structure :default "AnyKey"))
  (bind _camerapawnref (Variables|References|GetCameraPawnRef))
  (bind _returnvalue (Transformation|GetActorRotation _camerapawnref))
  (bind (_roll _pitch _yaw) (Math|Rotator|BreakRotator _returnvalue))
  ;[0.5198 0.8997 1] Camera Movement
  ;;[1 1 1] Pan Reset
  (:Pressed
    (Transformation|SetActorRotation _camerapawnref (Math|Rotator|MakeRotator _roll 0.0 _yaw))))

(event Input|ActionEvents|InputActionLockCamera
  (params (Key :type Key%20Structure :default "AnyKey"))
  ;[0.5198 0.8997 1] Camera Movement
  (:Pressed
    (if (Variables|Camera|GetdisableCamNav)
      (Variables|Camera|SetdisableCamNav false)
      (else
        (Variables|Camera|SetdisableCamNav true)))))

(event Input|ActionEvents|InputActionZoomIn
  (params (Key :type Key%20Structure :default "AnyKey"))
  (bind _camerapawnref (Variables|References|GetCameraPawnRef))
  (bind _springarm (Variables|/Game/RTS_Tutorial/Blueprints/CameraPawn.CameraPawn_C|GetSpringArm _camerapawnref))
  ;[0.5198 0.8997 1] Camera Movement
  ;;[1 1 1] Zoom In/Out
  (:Pressed
    (Variables|/Script/Engine.SpringArmComponent|SetTargetArmLength _springarm (Math|Float|Clamp(Float) (- (Variables|/Script/Engine.SpringArmComponent|GetTargetArmLength _springarm) (Variables|Camera|GetzoomSensitivity)) 5e+02 (Variables|Camera|GetmaxArmDistance)))))

(event Input|ActionEvents|InputActionDeselect
  (params (Key :type Key%20Structure :default "AnyKey"))
  ;[1 1 1] Get out of Building Mode
  (:Pressed
    (if (Variables|Building|GetbuildModeActive)
      (Default|KillGhost (Variables|References|GetGhostBuildingRef))
      (Variables|Building|SetbuildModeActive false))))

(event Input|AxisEvents|InputAxisMoveForward
  (params (AxisValue :type Float%20%28single-precision%29))
  ;[0.5198 0.8997 1] Camera Movement
  ;;[1 1 1] Movement X
  (if (not (Variables|Camera|GetdisableCamNav))
    (Transformation|SetActorTransform (Variables|References|GetCameraPawnRef) (Utilities|MovementX (CallFunction|MovementSpeedCalculation) (Variables|Default|GetfastMoveMultiplier) AxisValue (Variables|References|GetCameraPawnRef)))))

(event Input|AxisEvents|InputAxisMoveRight
  (params (AxisValue :type Float%20%28single-precision%29))
  (bind _movesensitivity (CallFunction|MovementSpeedCalculation))
  (bind _fastmovemultiplier (Variables|Default|GetfastMoveMultiplier))
  (bind _camerapawnref (Variables|References|GetCameraPawnRef))
  (bind _transfom (Utilities|MovementY AxisValue _movesensitivity _fastmovemultiplier _camerapawnref))
  (bind (_location _rotation _scale) (Math|Transform|BreakTransform _transfom))
  (bind (_x _y) (Math|Vector|BreakVector _location))
  ;[0.5198 0.8997 1] Camera Movement
  ;;[1 1 1] Movement Y
  (if (not (Variables|Camera|GetdisableCamNav))
    (Transformation|SetActorTransform (Variables|References|GetCameraPawnRef) (Math|Transform|MakeTransform (Math|Vector|MakeVector _x _y 0.0) _rotation _scale))))

(event Input|MouseEvents|MouseX
  (params (AxisValue :type Float%20%28single-precision%29))
  (bind _camerapawnref (Variables|References|GetCameraPawnRef))
  (bind _returnvalue (Transformation|GetActorRotation _camerapawnref))
  (bind (_roll _pitch _yaw) (Math|Rotator|BreakRotator _returnvalue))
  ;[0.5198 0.8997 1] Camera Movement
  ;;[1 1 1] Pan X
  (Utilities|FlowControl|Gate true
    (:Exit
      (Transformation|SetActorRotation (Variables|References|GetCameraPawnRef) (Math|Rotator|MakeRotator _roll _pitch (+ _yaw (* (Variables|Camera|GetpanSensitivity) AxisValue)))))))

(event Input|MouseEvents|MouseY
  (params (AxisValue :type Float%20%28single-precision%29))
  (bind _camerapawnref (Variables|References|GetCameraPawnRef))
  (bind _returnvalue (Transformation|GetActorRotation _camerapawnref))
  (bind (_roll _pitch _yaw) (Math|Rotator|BreakRotator _returnvalue))
  ;[0.5198 0.8997 1] Camera Movement
  ;;[1 1 1] Pan Y
  (Utilities|FlowControl|Gate true
    (:Exit
      (Transformation|SetActorRotation (Variables|References|GetCameraPawnRef) (Math|Rotator|MakeRotator _roll (Math|Float|Clamp(Float) (+ _pitch (* (Variables|Camera|GetpanSensitivity) AxisValue)) -15.0 45.0) _yaw)))))

(event Input|MouseEvents|MouseX
  (params (AxisValue :type Float%20%28single-precision%29))
  ;[0.5198 0.8997 1] Camera Movement
  ;;[1 1 1] Edge Movement
  (if (not (Variables|Camera|GetdisableCamNav))
    (bind (_deltaxspeed _deltayspeed) (Utilities|ScreenEdgeMovement))
    (Transformation|AddActorLocalOffset (Variables|References|GetCameraPawnRef) (Math|Vector|MakeVector _deltayspeed _deltaxspeed 0.0) true false)))

(event Input|MouseEvents|MouseY
  (params (AxisValue :type Float%20%28single-precision%29))
  ;[0.5198 0.8997 1] Camera Movement
  ;;[1 1 1] Edge Movement
  (if (not (Variables|Camera|GetdisableCamNav))
    (Utilities|ScreenEdgeMovement) ; enters at Mouse Y
  ))

(event Input|KeyboardEvents|LeftShift
  (params (Key :type Key%20Structure :default "AnyKey"))
  ;[0.5198 0.8997 1] Camera Movement
  ;;[1 1 1] Move Multiplier
  (:Pressed
    (Variables|Default|SetfastMoveMultiplier 2.0))
  (:Released
    (Variables|Default|SetfastMoveMultiplier 1.0)))

(event Input|MouseEvents|LeftMouseButton
  (params (Key :type Key%20Structure :default "AnyKey"))
  ;[1 1 1] Left Mouse Button
  (:Pressed
    (Utilities|FlowControl|Sequence
      (:then_0
        (if (|VerifyAsPlaceable)
          (bind _constructionstruct (Default|GetConstructionStruct (Variables|References|GetGhostBuildingRef)))
          (Default|QueueConstruction (Variables|References|GetConstructionManagerRef) _constructionstruct)
          (Default|KillGhost (Variables|References|GetGhostBuildingRef))))
      (:then_1
        (CallFunction|StartClick))))
  (:Released
    (Variables|Mouse|SetstartMousePosition "")
    (Variables|Mouse|SetendMousePosition "(X=0.000000,Y=0.000000)")))

(event Input|KeyboardEvents|I
  (params (Key :type Key%20Structure :default "AnyKey"))
  (bind _baseplayer (Variables|References|GetbasePlayer))
  (bind _heroes (Variables|/Script/MyProject.BasePlayer|Getheroes _baseplayer))
  ;[1 1 1] Inventory
  (:Pressed
    (bind _index (Utilities|FlowControl|ForLoopwithBreak 0 (Utilities|Array|Length _heroes) :!label _label)
      (:LoopBody
        (if (not (Class|Unit|GetSelected (Utilities|Array|Get(acopy) _heroes _index)))
          (Class|BaseHero|ToggleInventory (Utilities|Array|Get(acopy) _heroes _index))
          (goto _label Break))))))

(event Input|MouseEvents|RightMouseButton
  (params (Key :type Key%20Structure :default "AnyKey"))
  (bind _baseplayer (Variables|References|GetbasePlayer))
  (bind _heroes (Variables|/Script/MyProject.BasePlayer|Getheroes _baseplayer))
  ;[1 1 1] Right Mouse Button
  (:Pressed
    (for _index (range 0 (- (Utilities|Array|Length _heroes) 1))
      (if (Class|Unit|GetSelected (Utilities|Array|Get(acopy) _heroes _index))
        (Class|BaseHero|Move (Utilities|Array|Get(acopy) _heroes _index) (CallFunction|SetCursorWorldPosition self (CallFunction|SetSightDistance)))))))

(event Input|KeyboardEvents|V
  (params (Key :type Key%20Structure :default "AnyKey"))
  (bind _self self)
  (bind _location (CallFunction|SetCursorWorldPosition _self 1e+04))
  ;[0.2886 0.236 1] Debug
  (:Pressed
    (Game|SpawnActorfromClass "/Game/RTS_Tutorial/Blueprints/AI/NPC_BP.NPC_BP_C" (Math|Transform|MakeTransform (Math|Vector|MakeVector (.x _location) (.y _location) 92.5)) "Undefined" 0 0)))

(fn ConstructionScript)

(fn MovementSpeedCalculation
  (return (Math|Float|Clamp(Float) (/ (Variables|/Script/Engine.SpringArmComponent|GetTargetArmLength (Variables|/Game/RTS_Tutorial/Blueprints/CameraPawn.CameraPawn_C|GetSpringArm (Variables|References|GetCameraPawnRef))) 1e+02) 5.0 2e+01)))

(fn SetSightDistance
  (return (+ (Variables|Default|GetsightDistance) (Variables|/Script/Engine.SpringArmComponent|GetTargetArmLength (Variables|/Game/RTS_Tutorial/Blueprints/CameraPawn.CameraPawn_C|GetSpringArm (Variables|References|GetCameraPawnRef))))))

(fn IsRect
  (return (Math|Vector|NotEqual(Vector) (Variables|Mouse|GetstartMousePosition) (Variables|Mouse|GetendMousePosition) 0.0001)))

(fn GetHitObject
  (bind (_worldlocation _worlddirection) (Game|Player|ConvertMouseLocationToWorldSpace))
  (bind _outhit (Collision|LineTraceForObjects _worldlocation (+ _worldlocation (* _worlddirection 5e+03)) (Utilities|Array|MakeArray "ObjectTypeQuery8" "ObjectTypeQuery7") false 0 "None"))
  (if (!= (.HitActor (Collision|BreakHitResult _outhit)) 0)
    (return (.HitActor (Collision|BreakHitResult _outhit)))
    (else
      (return 0))))

(fn UpdateFadeActors
  (Utilities|Array|Clear (Variables|Fade|GethitMeshes))
  (bind _array_element (Utilities|HeroLoop)
    (:LoopBody
      (bind (_hits _returnvalue) (Class|BaseHero|GetOverlappingObjects _array_element))
      (if _returnvalue
        (for _array_element_2 _hits
          (if (!= 0 (Utilities|GetClass (.HitActor (Collision|BreakHitResult _array_element_2))))
            (bind _asstatic_mesh_actor (Utilities|Casting|CastToStaticMeshActor (.HitActor (Collision|BreakHitResult _array_element_2))))
            (Utilities|Array|AddUnique (Variables|Fade|GethitMeshes) _asstatic_mesh_actor)
            (CallFunction|SetShownMeshes)
            (CallFunction|SetHiddenMeshes)))
        (else
          (CallFunction|SetShownMeshes))))))

(fn SetShownMeshes
  (for _array_element (Variables|Fade|GethiddenMeshes)
    (if (not (Utilities|Array|ContainsItem (Variables|Fade|GethitMeshes) _array_element))
      (if (!= (Actor|GetComponentbyClass _array_element "/Game/RTS_Tutorial/Blueprints/Fade/BP_FadeComponent.BP_FadeComponent_C") 0)
        (Default|ToggleHideMesh (Actor|GetComponentbyClass _array_element "/Game/RTS_Tutorial/Blueprints/Fade/BP_FadeComponent.BP_FadeComponent_C") false)))))

(fn SetHiddenMeshes
  (bind _output_get (Variables|Fade|SethiddenMeshes (Variables|Fade|GethitMeshes)))
  (for _array_element _output_get
    (if (!= 0 (Utilities|GetClass (Actor|GetComponentbyClass _array_element "/Game/RTS_Tutorial/Blueprints/Fade/BP_FadeComponent.BP_FadeComponent_C")))
      (Default|ToggleHideMesh (Actor|GetComponentbyClass _array_element "/Game/RTS_Tutorial/Blueprints/Fade/BP_FadeComponent.BP_FadeComponent_C") true))))

(fn SetCalendar
  (params (Date :type Array%20of%20Integers))
  (return false))

(fn SetClock
  (params (Time :type Array%20of%20Integers))
  (return false))