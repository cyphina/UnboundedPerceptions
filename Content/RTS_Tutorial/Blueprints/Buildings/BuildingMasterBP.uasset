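; Master building Blueprint for an RTS that sets up its display mesh, entrance and collision box, and creates its own Building_HUD widget on BeginPlay.
; When DisplayHUD targets this actor, it shows that HUD, switches to UI-only input, and disables camera navigation and the in-game HUD.
; A LerpLocation timeline also drives the camera pawn through HUDLerp, though both endpoints read the pawn's current location.
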(event Custom|DisplayHUD
  (params (actor :type Actor%20Object%20Reference))
  (bind _controllerref (Variables|References|GetControllerRef))
  ;[1 1 1] Is this actor selecting me?
  (if (== actor self)
    (Utilities|FlowControl|Sequence
      (:then_0
        ;;[1 1 1] Camera Move to Selected
        (bind _newlocation (|LerpLocation)
          (:Update
            (Transformation|SetActorLocation (Class|UserInput|GetCameraPawn (Variables|References|GetControllerRef)) _newlocation false false))))
      (:then_1
        (UserInterface|Viewport|AddtoViewport (Variables|Default|GetbuildingHUD) 0)
        (Input|SetInputModeUIOnly _controllerref 0 "LockOnCapture")
        (Variables|/Script/MyProject.RTSPawn|SetisCamNavDisabled (Class|UserInput|GetCameraPawn _controllerref) true)
        (Widget|SetIsEnabled (Class|HUDManager|GetIngameHUD (Default|GetHudManager _controllerref)) false)))))

(event EventBeginPlay
  (bind _ascamera_pawn_controller (Utilities|Casting|CastToCameraPawnController (Game|GetPlayerController 0)))
  (Variables|References|SetControllerRef _ascamera_pawn_controller)
  (bind _returnvalue (UserInterface|CreateWidget "/Game/RTS_Tutorial/HUDs/BuildingUI/Building_HUD.Building_HUD_C" 0 self (Variables|References|GetControllerRef)))
  (Variables|Default|SetbuildingHUD _returnvalue)
  (Components|StaticMesh|SetStaticMesh (Variables|Default|GetStaticMesh) (Variables|Default|GetDisplayMesh))
  (CallFunction|SetBuildingEntrance (Variables|Default|GetEntrance) (Variables|Default|GetStaticMesh))
  (CallFunction|SetBuildingCollisionBox (Variables|Default|GetCollision) (Variables|Default|GetStaticMesh)))

(fn ConstructionScript)