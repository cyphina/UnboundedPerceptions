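; Pawn for the RTS tutorial's drawing minigame, letting the player paint on a spawned canvas with the mouse.
; Starting the minigame spawns BP_Canvas above the pawn and adds the HUDFinishedDrawing widget.
; The Paint axis traces from the cursor and converts canvas hits to UVs for brush strokes, while left mouse brackets each drawing action.
; Ending returns the canvas's drawing check result and removes both canvas and widget.
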(event EventBeginPlay)

(event Collision|EventActorBeginOverlap
  (params (OtherActor :type Actor%20Object%20Reference)))

(event EventTick
  (params (DeltaSeconds :type Float%20%28single-precision%29)))

(event EventStartMinigame
  (CallFunction|StartMG))

(event Input|AxisEvents|InputAxisPaint
  (params (AxisValue :type Float%20%28single-precision%29))
  (bind _returnvalue (Game|GetPlayerController 0))
  (bind (_worldlocation _worlddirection) (Game|Player|ConvertMouseLocationToWorldSpace _returnvalue))
  (if (== AxisValue 1.0)
    (bind _outhit (Collision|LineTraceByChannel _worldlocation (+ _worldlocation (* _worlddirection (* (Variables|/Script/Engine.SpringArmComponent|GetTargetArmLength (Variables|Default|GetSpringArm)) 3.0))) "TraceTypeQuery1" true 0 "None"))
    (if (== (Utilities|GetClass (.HitActor (Collision|BreakHitResult _outhit))) "/Game/RTS_Tutorial/Blueprints/Minigames/DrawingMinigame/BP_Canvas.BP_Canvas_C")
      (Default|DrawBrush (Variables|Default|GetcanvasRef) (Variables|Default|GetbrushSize) (.UV (Class|GameplayStatics|FindCollisionUV _outhit))))))

(event Input|MouseEvents|LeftMouseButton
  (params (Key :type Key%20Structure))
  (bind _canvasref (Variables|Default|GetcanvasRef))
  (:Pressed
    (Default|StartDrawing _canvasref (Variables|Default|GetbrushTexture)))
  (:Released
    (Default|FinishDrawing _canvasref)))

(fn ConstructionScript)

(fn EndMG
  (if (Class|MinigameCanvas|CheckDrawing (Variables|Default|GetcanvasRef))
    (Widget|RemovefromParent (Variables|Default|GetminigameWidgetRef))
    (Actor|DestroyActor (Variables|Default|GetcanvasRef))
    (return true)
    (else
      (Widget|RemovefromParent (Variables|Default|GetminigameWidgetRef))
      (Actor|DestroyActor (Variables|Default|GetcanvasRef))
      (return false))))

(fn StartMG
  (bind _returnvalue (Game|SpawnActorfromClass "/Game/RTS_Tutorial/Blueprints/Minigames/DrawingMinigame/BP_Canvas.BP_Canvas_C" (Math|Transform|MakeTransform (+ (Transformation|GetActorLocation) "0.000000, 0,200.000000") "0, 0, 0" (Math|Vector|MakeVector 1e+01 1e+01 1e+01)) "Undefined" self 0))
  (Variables|Default|SetcanvasRef _returnvalue)
  (bind _returnvalue_2 (UserInterface|CreateWidget "/Game/RTS_Tutorial/HUDs/MiniGames/HUDFinishedDrawing.HUDFinishedDrawing_C" 0 self))
  (Variables|Default|SetminigameWidgetRef _returnvalue_2)
  (UserInterface|Viewport|AddtoViewport _returnvalue_2 0))

(fn EndMinigame
  (bind _bminigamesuccess (CallFunction|EndMG))
  (return _bminigamesuccess))