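; BP_Canvas is a paintable canvas actor for a drawing minigame that draws brush strokes into a render target.
; On BeginPlay it gives its mesh a dynamic material showing the render target, creates a brush material, and stamps a starting picture onto the target.
; StartDrawing sets the brush texture and opens the render target for drawing, DrawBrush stamps the brush centered on a normalized location, and FinishDrawing closes the draw context.
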(event EventBeginPlay
  (Utilities|FlowControl|Sequence
    (:then_0
      (bind _returnvalue (Rendering|Material|CreateDynamicMaterialInstance "/Game/RTS_Tutorial/Blueprints/Minigames/DrawingMinigame/MAT_Canvas.MAT_Canvas" "None" :!class /Script/Engine.KismetMaterialLibrary))
      (Rendering|Material|SetTextureParameterValue _returnvalue "RenderTarget" (Variables|Default|GetrenderTarget))
      (Rendering|Material|SetMaterial (Variables|Default|GetcanvasMesh) 0 _returnvalue)
      (Variables|Default|SetcanvasMaterial _returnvalue))
    (:then_1
      (bind _returnvalue_2 (Rendering|Material|CreateDynamicMaterialInstance "/Game/RTS_Tutorial/Blueprints/Minigames/DrawingMinigame/M_Brush.M_Brush" "None" :!class /Script/Engine.KismetMaterialLibrary))
      (Variables|Default|SetbrushMaterial _returnvalue_2)
      (CallFunction|StartDrawing "/Game/RTS_Tutorial/Textures/catminigame.catminigame")
      (Canvas|DrawMaterial :self (Variables|Default|GetcanvasRef) :RenderMaterial "/Game/RTS_Tutorial/Blueprints/Minigames/DrawingMinigame/CanvasStartPicture.CanvasStartPicture" :ScreenPosition "(X=0.000000,Y=0.000000)" :ScreenSize "(X=1024.000000,Y=1024.000000)")
      (CallFunction|FinishDrawing))))

(fn ConstructionScript)

(fn DrawBrush
  (params (brushSize :type Float%20%28single-precision%29) (drawLocation :type Vector%202D%20Structure))
  (Canvas|DrawMaterial :self (Variables|Default|GetcanvasRef) :RenderMaterial (Variables|Default|GetbrushMaterial) :ScreenPosition (- (* (Variables|Default|GetcanvSize) drawLocation) (/ brushSize 2.0)) :ScreenSize (Math|Vector2D|MakeVector2D brushSize brushSize) :CoordinateSize "(X=1.000000,Y=1.000000)"))

(fn FinishDrawing
  (Rendering|EndDrawCanvastoRenderTarget (Variables|Default|GetdrawOperationContext)))

(fn StartDrawing
  (params (brushTex :type Texture%20Object%20Reference))
  (Rendering|Material|SetTextureParameterValue (Variables|Default|GetbrushMaterial) "BrushTexture" brushTex)
  (bind (_canvas _size _context) (Rendering|BeginDrawCanvastoRenderTarget (Variables|Default|GetrenderTarget)))
  (Variables|Default|SetcanvSize _size)
  (Variables|Default|SetcanvasRef _canvas)
  (Variables|Default|SetdrawOperationContext _context)
  (return))