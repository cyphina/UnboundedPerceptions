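; RTS camera pawn player controller that adds the in-game HUD on BeginPlay and hides meshes overlapping the heroes' view.
; Outside the starting level, a looping timer gathers BP_FadeComponent actors from each hero's overlap query, then diffs them against the hidden list to toggle visibility.
; It also provides cursor trace helpers, fade-timer pause/resume, a screen fade through a material parameter collection and initial dialog topics.
; The Z key is a debug hero knockback.
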(event Custom|Cyphina
  (Class|WidgetBlueprintLibrary|SetFocustoGameViewport)
  (Class|GameplayStatics|SetViewportMouseCaptureMode "CapturePermanently")
  (Development|PrintString "Hello"))

(event Custom|ScreenFade
  (bind _newtrack_0 (Timeline|fadeTimeline ReverseFromEnd)
    (:Update
      (Rendering|Material|SetScalarParameterValue "/Game/RTS_Tutorial/Materials/UIMats/TransitionMat/amount_paraCollection.amount_paraCollection" "amount" _newtrack_0 :!class /Script/Engine.KismetMaterialLibrary))))

(event EventBeginPlay
  ;[0 0 0] This is where all the things that pertain to starting up the game go
  (Utilities|FlowControl|Sequence
    (:then_0
      (|CallParentFunction)
      (Class|WidgetToggler|AddHUD (Class|UserInput|GetHUDManager) "HS_Ingame"))
    (:then_1
      (bind _returnvalue (Game|GetCurrentLevelName true)) ; If we're not on starting level
      (if (Utilities|Enum|NotEqual(Enum) _returnvalue (Class|RTSGameMode|GetStartingLvlName (Class|UserInput|GetGameMode)))
        (bind _returnvalue_2 (Utilities|Time|SetTimerbyFunctionName 0 "UpdateFadeActors" 0.1 true)) ; Setup a timer so we don't have to constantly check update
        (Variables|Default|SettimerHandleFade _returnvalue_2)))))

(event Input|KeyboardEvents|Z
  (params (Key :type Key%20Structure))
  (bind _returnvalue (Class|UpFunctionLibrary|GetHeroes))
  (bind _output (Utilities|Array|Get(acopy) _returnvalue))
  (bind _returnvalue_2 (Class|Unit|GetUnitController _output))
  (:Pressed
    (Development|PrintString "Hello")
    (Class|UnitController|PauseCurrentMovement _returnvalue_2)
    (Character|LaunchCharacter _output (* (Math|Vector|GetForwardVector (Variables|/Script/Engine.Character|GetCapsuleComponent _output)) -1000) true true)
    (Utilities|FlowControl|Delay 0.1)
    (Class|UnitController|ResumeCurrentMovement _returnvalue_2)))

(fn ConstructionScript)

(fn GetHitObjectActor
  (bind (_worldlocation _worlddirection) (Game|Player|ConvertMouseLocationToWorldSpace))
  (bind _outhit (Collision|LineTraceForObjects _worldlocation (+ _worldlocation (* _worlddirection (* (Variables|Camera|GetmaxArmDistance) 3.0))) (Utilities|Array|MakeArray "ObjectTypeQuery7" "ObjectTypeQuery12" "ObjectTypeQuery1" "ObjectTypeQuery8" "ObjectTypeQuery9") false 0 "None"))
  (if (!= (.HitActor (Collision|BreakHitResult _outhit)) 0)
    (return (.HitActor (Collision|BreakHitResult _outhit)))
    (else
      (return 0))))

(fn UpdateFadeActors
  (Utilities|Array|Clear (Variables|Fade|GethitMeshes))
  (bind _array_element (Utilities|HeroLoop :!label _label)
    (:LoopBody
      (if (Utilities|IsValid _array_element)
        (if (.ReturnValue (Class|Ally|GetOverlappingObjects _array_element))
          (for _array_element_2 (.hits (Class|Ally|GetOverlappingObjects _array_element))
            (if (Utilities|IsValidClass (Utilities|GetClass (.HitActor (Collision|BreakHitResult _array_element_2))))
              (if (!= (Actor|GetComponentbyClass (.HitActor (Collision|BreakHitResult _array_element_2)) "/Game/RTS_Tutorial/Blueprints/Effects/Fade/BP_FadeComponent.BP_FadeComponent_C") 0)
                (Utilities|Array|AddUnique (Variables|Fade|GethitMeshes) (.HitActor (Collision|BreakHitResult _array_element_2))) ; Generate list of hit meshes for all units
              ))))
        (else
          (goto _label Break))))
    (:Completed
      (Fade|SetShownMeshes) ; Look at our list of already hidden meshes\nand if any of them are not hit anymore, then\nthey are now visible
      (Fade|SetHiddenMeshes) ; Create a list of all meshes that are hidden
    )))

(fn SetShownMeshes
  ;[1 1 1] For each mesh, set each mesh to Not Hidden.  This is done when leaving a hidden mesh, so we have to check to see the tick when the hit mesh is finally not in hidden meshes.  We keep track of the hidden meshes so once the hit meshes don't correspond to hidden, we make it visible again
  (for _array_element (Variables|Fade|GethiddenMeshes)
    (if (not (Utilities|Array|ContainsItem (Variables|Fade|GethitMeshes) _array_element))
      (if (!= (Actor|GetComponentbyClass _array_element "/Game/RTS_Tutorial/Blueprints/Effects/Fade/BP_FadeComponent.BP_FadeComponent_C") 0) ; Some kind of null reference here not sure why
        (Default|ToggleHideMesh (Actor|GetComponentbyClass _array_element "/Game/RTS_Tutorial/Blueprints/Effects/Fade/BP_FadeComponent.BP_FadeComponent_C") false)))))

(fn SetHiddenMeshes
  ;[1 1 1] For each component, go set each mesh to "HIDDEN"
  (bind _output_get (Variables|Fade|SethiddenMeshes (Variables|Fade|GethitMeshes)))
  (for _array_element _output_get
    (if (!= 0 (Utilities|GetClass (Actor|GetComponentbyClass _array_element "/Game/RTS_Tutorial/Blueprints/Effects/Fade/BP_FadeComponent.BP_FadeComponent_C")))
      (Default|ToggleHideMesh (Actor|GetComponentbyClass _array_element "/Game/RTS_Tutorial/Blueprints/Effects/Fade/BP_FadeComponent.BP_FadeComponent_C") true))))

(fn GetHitObjectType
  (bind _array (Utilities|Array|MakeArray "ObjectTypeQuery9" "ObjectTypeQuery7" "ObjectTypeQuery8" "ObjectTypeQuery2" "ObjectTypeQuery1" "ObjectTypeQuery11" "ObjectTypeQuery13"))
  (bind _hitresult (Class|PlayerController|GetHitResultUnderCursorforObjects _array true))
  (bind (_bblockinghit _binitialoverlap _time _distance _location _impactpoint _normal _impactnormal _physmat _hitactor _hitcomponent) (Collision|BreakHitResult _hitresult))
  (bind _returnvalue (!= _hitactor 0))
  (if _returnvalue
    (return (Collision|GetCollisionObjectType _hitcomponent) _returnvalue)
    (else
      (return "ECC_WorldStatic" false))))

(fn PauseTimedFunctions
  (Utilities|Time|PauseTimerbyHandle (Variables|Default|GettimerHandleFade)))

(fn UnpauseTimedFunctions
  (Utilities|Time|UnpauseTimerbyHandle (Variables|Default|GettimerHandleFade)))