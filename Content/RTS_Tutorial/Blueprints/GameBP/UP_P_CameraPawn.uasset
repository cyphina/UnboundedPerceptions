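; RTS camera pawn Blueprint that handles player input helpers and cursor feedback on top of its parent class.
; Input toggles an occlusion radius through a material parameter collection, fading through the game state, and chat through the HUD manager.
; It spawns a spell circle shown at the cursor and time-stamped click decals.
; Functions trace under the mouse and move allies to group or split; selection-rectangle logic is disconnected.
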(event EventBeginPlay
  (|CallParentFunction)
  (Transformation|SetActorRotation "0,-180.000000, 0")
  (bind _returnvalue (Game|SpawnActorfromClass "/Game/RTS_Tutorial/Blueprints/Actors/Up_A_SpellCircle.Up_A_SpellCircle_C" (Math|Transform|MakeTransform "0, 0, 0" "0, 0, 0" "1,1,1") "Undefined" 0 (Variables|Default|GetcontrollerRef) 0))
  (Variables|Default|SetspellIndicator _returnvalue)
  (bind _asmy_game_state (Utilities|Casting|CastToMyGameState (Game|GetGameState)))
  (Variables|Default|SetMyGameStateRef _asmy_game_state))

(event EventShowSpellCircle
  (params (AOE :type Float%20%28single-precision%29))
  ;[1 0.1982 0.3483] Mouse effects
  (Default|Show (Variables|Default|GetspellIndicator) (CallFunction|GetCursorWorldPosition (Variables|Default|GetcontrollerRef) 5e+03) AOE))

(event EventHideSpellCircle
  ;[1 0.1982 0.3483] Mouse effects
  (Default|Hide (Variables|Default|GetspellIndicator)))

(event EventCreateClickVisual
  (params (visualLocation :type Vector :default "0, 0, 0"))
  ;[1 0.1982 0.3483] Mouse effects
  (Utilities|ClickVisual visualLocation))

(event Input|ActionEvents|InputActionToggleFade
  (params (Key :type Key%20Structure :default "None"))
  (:Pressed
    (bind _asmy_game_state (Utilities|Casting|CastToMyGameState (Game|GetGameState)))
    (Default|ToggleFade _asmy_game_state)))

(event Input|ActionEvents|InputActionChat
  (params (Key :type Key%20Structure :default "None"))
  (:Pressed
    (CallFunction|ChatboxControl)))

(event Input|ActionEvents|InputActionToggleOcclusion
  (params (Key :type Key%20Structure :default "None"))
  (:Pressed
    (if (Variables|Default|GetbOcclusionOn?)
      (Rendering|Material|SetScalarParameterValue "/Game/RTS_Tutorial/Materials/OcclusionMasking/Occlusion_MPC.Occlusion_MPC" "Radius" 0.0 :!class /Script/Engine.KismetMaterialLibrary)
      (else
        (Rendering|Material|SetScalarParameterValue "/Game/RTS_Tutorial/Materials/OcclusionMasking/Occlusion_MPC.Occlusion_MPC" "Radius" 8e+02 :!class /Script/Engine.KismetMaterialLibrary)))
    (Variables|Default|SetbOcclusionOn? (not (Variables|Default|GetbOcclusionOn?)))))

(event Input|ActionEvents|InputActionDeactivateChat
  (params (Key :type Key%20Structure :default "None"))
  (bind _controllerref (Variables|Default|GetcontrollerRef))
  (bind _returnvalue (Class|UserInput|GetHUDManager _controllerref))
  (:Pressed
    (if (Class|WidgetToggler|IsWidgetonScreen _returnvalue "HS_Ingame")
      (Class|WidgetToggler|AddHUD _returnvalue (Utilities|Enum|LiteralenumEHUDs "HS_ChatBox")))))

(event Input|MouseEvents|LeftMouseButton
  (params (Key :type Key%20Structure :default "None")))

(fn ConstructionScript
  (|CallParentFunction))

(fn GetHitObjectActor
  (bind _controllerref (Variables|Default|GetcontrollerRef))
  (bind (_worldlocation _worlddirection) (Game|Player|ConvertMouseLocationToWorldSpace _controllerref))
  (bind _outhit (Collision|LineTraceByChannel _worldlocation (+ _worldlocation (* _worlddirection (* (Class|RTSPawn|GetMaxArmLength) 3.0))) "TraceTypeQuery4" false 0 "None"))
  (if (!= (.HitActor (Collision|BreakHitResult _outhit)) 0)
    (return (.HitActor (Collision|BreakHitResult _outhit)))
    (else
      (return 0))))

(fn GetActorsinSelectionRect)

(fn Split
  (bind _controllerref (Variables|Default|GetcontrollerRef))
  (bind _returnvalue (Class|UserInput|GetBasePlayer _controllerref))
  (bind _allies (Variables|/Script/MyProject.BasePlayer|Getallies _returnvalue))
  (for _array_element _allies
    (LocalVariables|SetcenterPoint (+ (LocalVariables|GetcenterPoint) (Transformation|GetActorLocation _array_element))))
  (bind _output_get (LocalVariables|SetcenterPoint (/ (LocalVariables|GetcenterPoint) (Utilities|Array|Length _allies))))
  (for _array_element_2 _allies
    (AI|Navigation|SimpleMovetoLocation (Class|Unit|GetUnitController _array_element_2) (* (Class|KismetMathLibrary|VectorNormal2D (- (Transformation|GetActorLocation _array_element_2) _output_get) 0.0001) 1000))))

(fn Group
  (bind _controllerref (Variables|Default|GetcontrollerRef))
  (bind _returnvalue (Class|UserInput|GetBasePlayer _controllerref))
  (bind _allies (Variables|/Script/MyProject.BasePlayer|Getallies _returnvalue))
  (for _array_element _allies
    (LocalVariables|SetcenterPoint (+ (LocalVariables|GetcenterPoint) (Transformation|GetActorLocation _array_element))))
  (bind _output_get (LocalVariables|SetcenterPoint (/ (LocalVariables|GetcenterPoint) (Utilities|Array|Length _allies))))
  (for _array_element_2 _allies
    (AI|Navigation|SimpleMovetoLocation (Class|Unit|GetUnitController _array_element_2) _output_get)))

(fn ChatboxControl
  (bind _controllerref (Variables|Default|GetcontrollerRef))
  (bind _returnvalue (Class|UserInput|GetHUDManager _controllerref))
  (if (Class|WidgetToggler|IsWidgetonScreen _returnvalue "HS_Ingame")
    (bind _asup_w_ingame_widget (Utilities|Casting|CastToUp_W_IngameWidget (Class|HUDProvider|GetIngameHUD _returnvalue)))
    (Default|SetFocus (Variables|/Script/MyProject.RTSIngameWidget|GetChatbox _asup_w_ingame_widget))
    (else
      (Class|WidgetToggler|AddHUD _returnvalue (Utilities|Enum|LiteralenumEHUDs "HS_ChatBox")))))