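; RTS game mode that manages streamed level transitions and shows the section-completed and game-over widgets.
; A transition shows a loading widget, then removes the current level: notifies listeners, destroys non-hero allies, saves via the game instance and unloads.
; A short delay before unloading works around race conditions from vision updates.
; The new level streams in, then the game pauses while saved data loads and a level-loaded notification fires.
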(event Custom|OnSectionCompleted
  (params (sectionName :type Gameplay%20Tag%20Structure))
  (bind _returnvalue (UserInterface|CreateWidget "/Game/RTS_Tutorial/HUDs/Loading/Up_W_NextSectionEffectWidget.Up_W_NextSectionEffectWidget_C" 0 (Variables|Default|GeteventManager)))
  (UserInterface|Viewport|AddtoViewport _returnvalue 1))

(event EventBeginPlay
  (|CallParentFunction)
  (EventDispatchers|AssignOnSectionCompletedDelegate (Variables|Default|GeteventManager) (delegate Custom|OnSectionCompleted))
  (bind _asrtsgame_instance (Utilities|Casting|CastToRTSGameInstance (Game|GetGameInstance)))
  (Variables|Default|SetgameInstanceRef _asrtsgame_instance)
  (bind _asrtsgame_state (Utilities|Casting|CastToRTSGameState (Game|GetGameState)))
  (Variables|Default|SetgameStateRef _asrtsgame_state))

(event EventGameOver
  (bind _returnvalue (UserInterface|CreateWidget "/Game/RTS_Tutorial/HUDs/MainUI/Up_W_GameOverWidget.Up_W_GameOverWidget_C"))
  (UserInterface|Viewport|AddtoViewport _returnvalue 0))

(event EventStreamLevelAsync
  (params (levelName :type Name :default "None"))
  (bind _currentlevelname (Variables|Default|GetcurrentLevelName))
  (bind _returnvalue (Utilities|String|StringToName _currentlevelname))
  (Variables|Default|SetnewLevelName levelName)
  (bind _returnvalue_2 (UserInterface|CreateWidget "/Game/RTS_Tutorial/HUDs/Loading/Up_W_LoadingWidget.Up_W_LoadingWidget_C")) ; Widget to show while new  level data is loading
  (bind _output_get (Variables|Default|SetloadingWidget _returnvalue_2))
  (UserInterface|Viewport|AddtoViewport _output_get 10)
  (if (Utilities|Name|NotEqual(Name) _returnvalue "None") ; If we're not in the start level
    (|HandleLevelRemoval _returnvalue
      (:Completed
        _)))
  (if (Utilities|Name|NotEqual(Name) (Variables|Default|GetnewLevelName) "None")
    (|HandleNewLevelEntry (Variables|Default|GetnewLevelName))))

(fn ConstructionScript)

(fn DeleteSummonedUnits
  (bind _ascamera_pawn_controller (Utilities|Casting|CastToCameraPawnController (Game|GetPlayerController 0)))
  (for _array_element (Variables|/Script/MyProject.BasePlayer|Getallies (Class|UserInput|GetBasePlayer _ascamera_pawn_controller))
    (if (not (Utilities|ClassIsChildOf (Utilities|GetClass _array_element) "/Script/MyProject.BaseHero")) ; If our unit is a summon (not a hero)
      (Utilities|Array|Add (LocalVariables|Getsummons) _array_element)))
  (for _array_element_2 (LocalVariables|Getsummons)
    (Actor|DestroyActor _array_element_2)))