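; Game state for the RTS tutorial that holds game-time and calendar helpers and a global toggle for fade components.
; Clock converts Clockwork seconds into time, and Calendar rolls the date over, but this file never calls either.
; Tick only runs the BLUI event loop.
; ToggleFade switches component ticking and the camera controller's fade timer with HUD text, though no live path here sets FadeOn back to true.
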(event EventBeginPlay
  ;[1 1 1] Startup
  (|CallParentFunction)
  (bind _ascamera_pawn_controller (Utilities|Casting|CastToCameraPawnController (Game|GetPlayerController 0)))
  (Variables|Default|SetControllerRef _ascamera_pawn_controller))

(event EventTick
  (params (DeltaSeconds :type Float%20%28single-precision%29))
  ;[1 1 1] Event tick gives the number of seconds passed between frames
  (|CallParentFunction DeltaSeconds)
  (Class|BluBlueprintFunctionLibrary|RunBluEventLoop))

(event EventEndPlay
  (params (EndPlayReason :type EEndPlayReason%20Enum :default "Destroyed"))
  (Utilities|Array|Clear (Variables|Default|GetfadeComponents)))

(fn ConstructionScript)

(fn Clock
  (bind _clockwork (Variables|Default|GetClockwork))
  (bind (_remainder _returnvalue) (Math|Float|Division(WholeandRemainder) _clockwork 6e+01))
  (bind _returnvalue_2 (Math|Conversions|ToFloat(Integer) _returnvalue))
  (bind (_remainder_2 _returnvalue_3) (Math|Float|Division(WholeandRemainder) _returnvalue_2 6e+01))
  (Variables|Default|SetSeconds (Math|Float|Floor _remainder)) ; Every 1/3600 value of clockwork increments set.
  (Variables|Default|SetMinutes (Math|Float|Floor _remainder_2))
  (Variables|Default|SetHours (Math|Float|Floor (.Remainder (Math|Float|Division(WholeandRemainder) (Math|Conversions|ToFloat(Integer) _returnvalue_3) 24.0))))
  (Variables|Default|SetGameTime (Utilities|Array|MakeArray (Variables|Default|GetSeconds) (Variables|Default|GetMinutes) (Variables|Default|GetHours))))

(fn Calendar
  (bind _output_get (Variables|Default|SetDay (+ (Variables|Default|GetDay) (Variables|Default|GetDayTick))))
  (if (> _output_get (Class|KismetMathLibrary|DaysinMonth (Variables|Default|GetYear) (Variables|Default|GetMonth)))
    (Variables|Default|SetDay 1)
    (Variables|Default|SetMonth (+ (Variables|Default|GetMonth) 1)))
  (if (> (Variables|Default|GetMonth) 12)
    (Variables|Default|SetMonth 1)
    (Variables|Default|SetYear (+ (Variables|Default|GetYear) 1)))
  (Variables|Default|SetGameDate (Utilities|Array|MakeArray (Variables|Default|GetDay) (Variables|Default|GetMonth) (Variables|Default|GetYear))))

(fn GetCurrentTimeUnit
  (return (Variables|Default|GetTimeUnit)))

(fn ToggleFade
  (bind _controllerref (Variables|Default|GetControllerRef))
  (bind _returnvalue (Class|UserInput|GetHUDManager _controllerref))
  (bind _returnvalue_2 (Class|HUDProvider|GetIngameHUD _returnvalue))
  (if (Variables|Default|GetFadeOn?)
    (for _array_element (Variables|Default|GetfadeComponents)
      (Default|StopFade _array_element)
      (Components|Tick|SetComponentTickEnabled _array_element false)
      (Class|KismetSystemLibrary|PauseTimer (Variables|Default|GetControllerRef) "UpdateFadeActors")
      (Class|RTSIngameWidget|DisplayHelpText _returnvalue_2 (Utilities|Text|MakeLiteralText "Fade Off"))
      (Variables|Default|SetFadeOn? false))
    (else
      (for _array_element_2 (Variables|Default|GetfadeComponents)
        (Components|Tick|SetComponentTickEnabled _array_element_2 true)
        (Class|KismetSystemLibrary|UnPauseTimer _controllerref "UpdateFadeActors")
        (Class|RTSIngameWidget|DisplayHelpText _returnvalue_2 (Utilities|Text|MakeLiteralText "Fade On"))))))