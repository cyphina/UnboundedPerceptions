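; An effect actor that publishes the direction of its DirectionalLight to materials through the LightSource Material Parameter Collection.
; It negates the light's forward vector, so it points back toward the light, and writes it to the DirectLight vector parameter.
; The write runs in both the Construction Script and BeginPlay, with no per-frame update for later rotation changes.
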(event EventBeginPlay
  (Rendering|Material|SetVectorParameterValue "/Game/RTS_Tutorial/Materials/CelShade/LightSource.LightSource" "DirectLight" (Math|Conversions|ToLinearColor(Vector) (* (Math|Vector|GetForwardVector (Variables|Default|GetDirectionalLight)) -1.0)) :!class /Script/Engine.KismetMaterialLibrary))

(event Collision|EventActorBeginOverlap
  (params (OtherActor :type Actor%20Object%20Reference)))

(fn ConstructionScript
  (Rendering|Material|SetVectorParameterValue "/Game/RTS_Tutorial/Materials/CelShade/LightSource.LightSource" "DirectLight" (Math|Conversions|ToLinearColor(Vector) (* (Math|Vector|GetForwardVector (Variables|Default|GetDirectionalLight)) -1.0)) :!class /Script/Engine.KismetMaterialLibrary))