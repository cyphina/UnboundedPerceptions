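; Actor component that fades its owner's static mesh out and back in when toggled hidden, registering itself with MyGameState.
; Hiding swaps every material slot to a shared dynamic fade material, whose opacity Tick drives through a curve while the owner is recently rendered.
; A fully faded mesh ignores a trace channel, while a fully restored one regains its materials and initial response.
; StopFade immediately restores materials and blocking.
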(event EventBeginPlay
  (bind _output_get (Variables|Default|SetparentMesh (Actor|GetComponentbyClass (Components|GetOwner) "/Script/Engine.StaticMeshComponent")))
  (for _array_element (Rendering|Material|GetMaterials _output_get)
    (bind _returnvalue (Rendering|Material|CreateDynamicMaterialInstance _array_element "None" :!class /Script/Engine.KismetMaterialLibrary))
    (Utilities|Array|Add (Variables|Default|GetBaseMaterials) _returnvalue))
  (bind _returnvalue_2 (Rendering|Material|CreateDynamicMaterialInstance (Variables|Default|GetFadeMaterial) "None" :!class /Script/Engine.KismetMaterialLibrary))
  (Variables|Default|SetFadeMaterialMID _returnvalue_2)
  (Collision|SetCollisionResponsetoChannel (Variables|Default|GetparentMesh) "ECC_GameTraceChannel12" "ECR_Overlap")
  (Variables|Default|SetgroundTraceInit (Collision|GetCollisionResponsetoChannel (Variables|Default|GetparentMesh) "ECC_GameTraceChannel1"))
  (bind _asmy_game_state (Utilities|Casting|CastToMyGameState (Game|GetGameState)))
  (Utilities|Array|Add (Variables|/Game/RTS_Tutorial/Blueprints/GameBP/MyGameState.MyGameState_C|GetfadeComponents _asmy_game_state) self))

(event EventTick
  (params (DeltaSeconds :type Float%20%28single-precision%29))
  (bind _parentmesh (Variables|Default|GetparentMesh))
  (if (Class|Actor|WasRecentlyRendered (Components|GetOwner) 0.1)
    (Variables|Default|SetdeltaTime DeltaSeconds)
    (if (Variables|Default|Gethidden)
      ;[1 1 1] Fade Away...
      (Variables|Default|SetcurrentFade (Math|Float|Clamp(Float) (- (Variables|Default|GetcurrentFade) (* (Variables|Default|GetdeltaTime) (Variables|Default|GetFadeRate)))))
      (else
        ;[1 1 1] Fade In...
        (Variables|Default|SetcurrentFade (Math|Float|Clamp(Float) (+ (Variables|Default|GetcurrentFade) (* (Variables|Default|GetdeltaTime) (Variables|Default|GetFadeRate)))))))
    (Rendering|Material|SetScalarParameterValue (Variables|Default|GetFadeMaterialMID) "Fade" (Math|Curves|GetFloatValue (Variables|Default|GetfadeCurve) (Variables|Default|GetcurrentFade)) :!class /Script/Engine.MaterialInstanceDynamic)
    (if (not (Variables|Default|Gethidden))
      (if (== (Variables|Default|GetcurrentFade) 1.0)
        (Utilities|FlowControl|Gate false :!label _label
          (:Exit
            (for _index (range 0 (- (Rendering|Material|GetNumMaterials _parentmesh) 1))
              (Rendering|Material|SetMaterial _parentmesh _index (Utilities|Array|Get(acopy) (Variables|Default|GetBaseMaterials) _index))
              (Collision|SetCollisionResponsetoChannel _parentmesh "ECC_GameTraceChannel1" (Variables|Default|GetgroundTraceInit))
              (goto _label Close))))
        (else
          (goto _label Open)))
      (elif (== (Variables|Default|GetcurrentFade) 0.0)
        (Utilities|FlowControl|Gate false :!label _label_2
          (:Exit
            (Collision|SetCollisionResponsetoChannel _parentmesh "ECC_GameTraceChannel1" "ECR_Ignore")
            (goto _label_2 Close)))
        (else
          (goto _label_2 Open))))))

(fn ToggleHideMesh
  (params (hidden :type Boolean))
  (bind _parentmesh (Variables|Default|GetparentMesh))
  (if (Math|Boolean|NotEqual(Boolean) hidden (Variables|Default|Gethidden))
    (bind _output_get (Variables|Default|Sethidden hidden))
    (if _output_get
      (for _index (range 0 (Rendering|Material|GetNumMaterials _parentmesh))
        (Rendering|Material|SetMaterial _parentmesh _index (Variables|Default|GetFadeMaterialMID))))))

(fn StopFade
  (bind _parentmesh (Variables|Default|GetparentMesh))
  (Rendering|Material|SetScalarParameterValue (Variables|Default|GetFadeMaterialMID) "Fade" 0.0 :!class /Script/Engine.MaterialInstanceDynamic)
  (Variables|Default|SetcurrentFade 0.0)
  (for (_array_element _array_index) (Variables|Default|GetBaseMaterials)
    (Rendering|Material|SetMaterial _parentmesh _array_index _array_element))
  (Collision|SetCollisionResponsetoChannel _parentmesh "ECC_GameTraceChannel1" "ECR_Block")
  (Variables|Default|Sethidden false))