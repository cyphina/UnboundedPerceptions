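; A cone-shaped damage volume actor that applies a supplied gameplay effect spec to actors while they overlap it.
; Overlap begin applies the spec through the actor's ability system component; overlap end removes active effects matching the name tag read from that spec at BeginPlay.
; The construction script orients and scales the cone from direction, range and radius, offsets it, sets overlap channels, scales particles and optionally applies a debug material.
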(event EventBeginPlay
  (bind _output_get (Variables|Default|SetEffectNameTag (Class|SpellDataLibrary|GetEffectNameTagfromSpec (Ability|GetAbilitySystemComponent (Game|GetInstigator)) (Variables|Default|GetEffectToApply))))
  (Development|PrintString (GameplayTags|GetDebugStringfromGameplayTag _output_get)))

(event Collision|EventActorBeginOverlap
  (params (OtherActor :type Actor%20Object%20Reference))
  (GameplayEffects|ApplyGameplayEffectSpecToSelf (Ability|GetAbilitySystemComponent OtherActor) (Variables|Default|GetEffectToApply)))

(event Collision|EventActorEndOverlap
  (params (OtherActor :type Actor%20Object%20Reference))
  (GameplayEffects|RemoveActiveEffectswithTags (Ability|GetAbilitySystemComponent OtherActor) (GameplayTags|MakeGameplayTagContainerfromTag (Variables|Default|GetEffectNameTag))))

(fn ConstructionScript
  (bind _cone (Variables|Default|GetCone))
  (bind _relativelocation (Variables|/Script/Engine.SceneComponent|GetRelativeLocation _cone))
  (Transformation|SetActorRotation (Math|Rotator|FindLookatRotation _relativelocation (+ _relativelocation (Variables|Default|GetDirection))))
  (LocalVariables|SetnewRange (/ (Variables|Default|GetRange) 1e+02))
  (LocalVariables|SetnewRadius (/ (Variables|Default|GetRadius) 5e+01))
  (Transformation|SetRelativeScale3D (Variables|Default|GetCone) (Math|Vector|MakeVector (LocalVariables|GetnewRadius) (LocalVariables|GetnewRadius) (LocalVariables|GetnewRange)))
  (Transformation|SetRelativeScale3D (Variables|Default|GetParticleSystem) (Variables|Default|GetParticleScale))
  (for _array_element (Variables|Default|GetObjectCollisionChannels)
    (Collision|SetCollisionResponsetoChannel (Variables|Default|GetCone) _array_element "ECR_Overlap")
    (Transformation|AddWorldOffset (Variables|Default|GetScene) (Math|Vector|MakeVector 0.0 0.0 (Variables|Default|GetZOffset)) false false)
    (Transformation|AddWorldOffset (Variables|Default|GetScene) (* (Math|Vector|GetUpVector (Variables|Default|GetCone)) (/ (Variables|Default|GetRange) -2.0)) false false)
    (if (Variables|Default|GetDebug)
      (Rendering|Material|SetMaterial (Variables|Default|GetCone) 0 "/Game/InfinityBladeEffects/Effects/FX_Materials/Misc/M_FlickerGlow_Forge_IB_INST.M_FlickerGlow_Forge_IB_INST"))))