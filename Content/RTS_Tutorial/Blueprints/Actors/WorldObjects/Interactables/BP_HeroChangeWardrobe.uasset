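; BP_HeroChangeWardrobe is an interactable world object that opens the party screen for changing heroes.
; Interact creates a PartyScreen widget and binds to its closed event.
; On close, it moves each of the base player's heroes, found through the cached CameraPawnController, to a random reachable navmesh point in front of the wardrobe, raised slightly above the ground.
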(event Custom|OnPartyScreenClosed_Event
  (for _array_element (Variables|/Script/MyProject.BasePlayer|Getheroes (Class|UserInput|GetBasePlayer (Variables|Default|GetcontrollerRef)))
    (Transformation|SetActorLocation _array_element (+ (.RandomLocation (AI|Navigation|GetRandomReachablePointinRadius (+ (Class|Interactable|GetInteractableLocation) (* (Transformation|GetActorForwardVector) 500)) 2.5e+02 0 "/Script/NavigationSystem.NavigationQueryFilter")) "0, 0,90.000000") false false)))

(event EventBeginPlay
  (|CallParentFunction)
  (bind _ascamera_pawn_controller (Utilities|Casting|CastToCameraPawnController (Game|GetPlayerController 0)))
  (Variables|Default|SetcontrollerRef _ascamera_pawn_controller))

(event Collision|EventActorBeginOverlap
  (params (OtherActor :type Actor%20Object%20Reference)))

(event EventTick
  (params (DeltaSeconds :type Float%20%28single-precision%29)))

(event EventInteract
  (params (hero :type Base%20Hero%20Object%20Reference))
  (bind _returnvalue (UserInterface|CreateWidget "/Game/RTS_Tutorial/HUDs/ActionUI/CharacterSwapMenu/PartyScreen.PartyScreen_C"))
  (EventDispatchers|AssignOnPartyScreenClosed _returnvalue (delegate Custom|OnPartyScreenClosed_Event))
  (UserInterface|Viewport|AddtoViewport _returnvalue 0))

(fn ConstructionScript)

(fn GetInteractableLocation
  (return (|CallParentFunction)))