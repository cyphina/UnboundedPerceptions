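; Base Blueprint for allied RTS heroes, owned by the player pawn, with level-up sound and particle feedback.
; BeginPlay hides the hero icon from its owner and drops the mesh by its bounds height.
; An unfinished line-of-sight prototype gathers nearby blocker corners, then debug-draws and traces between corner pairs.
; Its call from the event graph, the barycentric enemy-hiding test and the quest-distance update on movement are all disconnected.
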(event Custom|Die_1)

(event EventBeginPlay
  (bind _mesh (Variables|Character|GetMesh))
  ;[1 1 1] BeginPlay Setup
  (|CallParentFunction)
  (Actor|SetOwner (Game|Player|GetPlayerPawn 0))
  (Class|PrimitiveComponent|SetOwnerNoSee (Variables|Default|GetHeroIcon) true)
  (Transformation|SetRelativeLocation _mesh (Math|Vector|MakeVector 0.0 0.0 (* (.z (.BoxExtent (Collision|GetComponentBounds _mesh))) -1.0)) false false))

(event EventTick
  (params (DeltaSeconds :type Float%20%28single-precision%29))
  ;[1 1 1] If our main character is moving, update the quest distance calculation
  (|CallParentFunction DeltaSeconds))

(event EventLevelUp
  ;[0.315 1 0.4792] Player Feedback
  (|CallParentFunction)
  (Audio|PlaySound2D "/Game/RTS_Tutorial/Blueprints/Quest/Audio/LevelUpSound.LevelUpSound" 0.1 0.2 0.0 0 0)
  (Effects|SpawnEmitteratLocation (Variables|Default|GetLevelUpEffect) (Transformation|GetActorLocation)))

(fn ConstructionScript)

(fn CalculateVision
  (bind _returnvalue (Transformation|GetActorLocation))
  ;[1 0.8031 0.3108 1 36] Get all the corners of visionblockers in range
  (bind _outactors (Collision|SphereOverlapActors (Transformation|GetActorLocation) (Components|Sphere|GetScaledSphereRadius (Variables|Default|GetvisionComponent)) (Utilities|Array|MakeArray "ObjectTypeQuery11") 0))
  (for _array_element _outactors
    (Utilities|Array|Clear (Variables|Default|GetInRangeCorners))
    (Utilities|Array|Clear (Variables|Default|GetEndOfVisibleTriangle))
    (for _array_element_2 (Variables|Default|GetCorners)
      (if (< (Math|Vector|VectorLengthSquared (- (Math|Vector|MakeVector (.x (+ (.Origin (Collision|GetActorBounds _array_element false false)) (* (.BoxExtent (Collision|GetActorBounds _array_element false false)) _array_element_2))) (.y (+ (.Origin (Collision|GetActorBounds _array_element false false)) (* (.BoxExtent (Collision|GetActorBounds _array_element false false)) _array_element_2))) (.z (Transformation|GetActorLocation))) (Transformation|GetActorLocation))) 1.44e+06)
        (Utilities|Array|Add (Variables|Default|GetEndOfVisibleTriangle) (Math|Float|Sqrt (/ 1.44e+06 (Math|Vector|VectorLengthSquared (- (Math|Vector|MakeVector (.x (+ (.Origin (Collision|GetActorBounds _array_element false false)) (* (.BoxExtent (Collision|GetActorBounds _array_element false false)) _array_element_2))) (.y (+ (.Origin (Collision|GetActorBounds _array_element false false)) (* (.BoxExtent (Collision|GetActorBounds _array_element false false)) _array_element_2))) (.z (Transformation|GetActorLocation))) (Transformation|GetActorLocation))))))
        (Utilities|Array|Add (Variables|Default|GetInRangeCorners) (- (Math|Vector|MakeVector (.x (+ (.Origin (Collision|GetActorBounds _array_element false false)) (* (.BoxExtent (Collision|GetActorBounds _array_element false false)) _array_element_2))) (.y (+ (.Origin (Collision|GetActorBounds _array_element false false)) (* (.BoxExtent (Collision|GetActorBounds _array_element false false)) _array_element_2))) (.z (Transformation|GetActorLocation))) (Transformation|GetActorLocation)))
        (Rendering|Debug|DrawDebugLine _returnvalue (+ (- (Math|Vector|MakeVector (.x (+ (.Origin (Collision|GetActorBounds _array_element false false)) (* (.BoxExtent (Collision|GetActorBounds _array_element false false)) _array_element_2))) (.y (+ (.Origin (Collision|GetActorBounds _array_element false false)) (* (.BoxExtent (Collision|GetActorBounds _array_element false false)) _array_element_2))) (.z (Transformation|GetActorLocation))) (Transformation|GetActorLocation)) _returnvalue) "(R=0.213542,G=0.000000,B=0.189890,A=1.000000)" 0.0 1e+01)))
    (CallFunction|InsideTriangleTest)))

(fn InsideTriangleTest
  (bind _returnvalue (Transformation|GetActorLocation))
  (bind _inrangecorners (Variables|Default|GetInRangeCorners))
  (bind _inrangecorners_2 (Variables|Default|GetInRangeCorners))
  (bind _returnvalue_2 (Utilities|Array|Length _inrangecorners))
  (if (> _returnvalue_2 0)
    (bind _index (Utilities|FlowControl|ForLoopwithBreak 1 (- _returnvalue_2 1))
      (:LoopBody
        (bind _output_get (LocalVariables|SetcurrentCornerIndex _index))
        (LocalVariables|SetV1 (Utilities|Array|Get(acopy) _inrangecorners_2 (- _output_get 1)))
        (LocalVariables|SetV2 (Utilities|Array|Get(acopy) _inrangecorners_2 _output_get))
        (Rendering|Debug|DrawDebugLine :LineStart _returnvalue :LineEnd (+ (+ (LocalVariables|GetV1) (LocalVariables|GetV2)) (Transformation|GetActorLocation)) :Thickness 1e+01)
        (bind _returnvalue_3 (Collision|LineTraceForObjects _returnvalue (+ (+ (LocalVariables|GetV1) (LocalVariables|GetV2)) (Transformation|GetActorLocation)) (Utilities|Array|MakeArray "ObjectTypeQuery11") false 0 "None"))))))