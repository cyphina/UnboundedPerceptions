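; Trigger box actor for the RTS tutorial that fires gameplay triggers and dialog when something overlaps it while its conditions are met.
; On overlap it halts the other actor's movement, then checks every listed condition through the game mode's ConditionalManager.
; On success it activates its triggers via the TriggerManager and queues its messages as chained HUD dialog lines.
; It can optionally destroy itself after succeeding.
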(event OnComponentBeginOverlap(Box)
  (params (OverlappedComponent :type Primitive%20Component%20Object%20Reference) (OtherActor :type Actor%20Object%20Reference) (OtherComp :type Primitive%20Component%20Object%20Reference) (OtherBodyIndex :type Integer) (bFromSweep :type Boolean) (SweepResult :type Hit%20Result%20Structure%20%28by%20ref%29))
  (Components|Movement|StopMovementImmediately (Actor|GetComponentbyClass OtherActor "/Script/Engine.CharacterMovementComponent"))
  (if (CallFunction|DoesMeetConditional?)
    (CallFunction|ActivateTriggers)
    (Class|WidgetToggler|AddHUDDialogString(Message) (Class|UserInput|GetHUDManager (Variables|Default|GetcontrollerRef)) (CallFunction|CreateDialogLines) "finishedTriggerActivation")
    ;[1 1 1] Destroy the actor if this barricade only checks once to see if conditions are fulfilled
    (if (Variables|Default|GetbIsDestroyedAfterSuccess)
      (Actor|DestroyActor))))

(event EventBeginPlay
  (bind _asuser_input (Utilities|Casting|CastToUserInput (Game|GetPlayerController 0)))
  (Variables|Default|SetcontrollerRef _asuser_input)
  (bind _asmy_rtsgame_mode (Utilities|Casting|CastToMyRTSGameMode (Game|GetGameMode)))
  (Variables|Default|SetgameModeRef _asmy_rtsgame_mode))

(event Collision|EventActorBeginOverlap
  (params (OtherActor :type Actor%20Object%20Reference)))

(event EventTick
  (params (DeltaSeconds :type Float%20%28single-precision%29)))

(fn ConstructionScript)

(fn CreateDialogLines
  (bind _messagenames (Variables|Default|GetmessageNames))
  (bind _activationmessage (Variables|Default|GetactivationMessage))
  (bind _dialoglines (LocalVariables|GetdialogLines))
  (bind _returnvalue (Utilities|Array|Length _activationmessage))
  (bind _returnvalue_2 (- _returnvalue 1))
  (if (> (Utilities|Array|Length (Variables|Default|GetactivationMessage)) 0)
    (for _index (range 0 (- _returnvalue 2))
      (Utilities|Array|Add (LocalVariables|GetdialogLines) (Utilities|Struct|MakeDialogData (Utilities|Array|MakeArray (+ _index 1)) (Utilities|Array|Get(acopy) _activationmessage _index) (Utilities|Array|Get(acopy) _messagenames _index))))
    (Utilities|Array|Add _dialoglines (Utilities|Struct|MakeDialogData (Utilities|Array|MakeArray) (Utilities|Array|Get(acopy) _activationmessage _returnvalue_2) (Utilities|Array|Get(acopy) _messagenames _returnvalue_2)))
    (return _dialoglines)
    (else
      (return (Utilities|Array|MakeArray)))))

(fn DoesMeetConditional?
  (for _array_element (Variables|Default|Getconditions)
    (if (not (Class|ConditionalManager|GetCondition (Variables|/Script/MyProject.RTSGameMode|GetconditionalManager (Variables|Default|GetgameModeRef)) _array_element))
      (return false)))
  (return true))

(fn ActivateTriggers
  (bind _arrayelement (Utilities|ForEachRef (Variables|Default|Gettriggers))
    (:then
      (Class|TriggerManager|ActivateTrigger (Variables|/Script/MyProject.RTSGameMode|GettriggerManager (Variables|Default|GetgameModeRef)) _arrayelement))))