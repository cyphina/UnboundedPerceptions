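; Event barricade trigger that blocks heroes from passing until a set of game conditions is met.
; When a hero overlaps the box, it checks each condition through the game mode's ConditionalManager, optionally destroying itself on success.
; On failure it moves the hero to a reset position, stops its current action and shows HUD dialog in that hero's name, using custom block lines or the failed condition's text.
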(event OnComponentBeginOverlap(Box)
  (params (OverlappedComponent :type Primitive%20Component%20Object%20Reference) (OtherActor :type Actor%20Object%20Reference) (OtherComp :type Primitive%20Component%20Object%20Reference) (OtherBodyIndex :type Integer) (bFromSweep :type Boolean) (SweepResult :type Hit%20Result%20Structure%20%28by%20ref%29))
  (bind _asbase_hero (Utilities|Casting|CastToBaseHero OtherActor))
  (if (CallFunction|DoesMeetConditional?)
    ;[1 1 1] Destroy the actor if this barricade only checks once to see if conditions are fulfilled
    (if (Variables|Default|GetbIsDestroyedAfterSuccess)
      (Actor|DestroyActor))
    (else
      ;[1 1 1] If the conditionals aren't fufilled, let a popup message occur and move passing character back to preset location
      (Transformation|SetActorLocation OtherActor (Variables|Default|GetresetPosition) false false)
      (Class|UnitController|StopCurrentAction (Class|Unit|GetUnitController _asbase_hero))
      (Class|WidgetToggler|AddHUDDialogString (Class|UserInput|GetHUDManager (Variables|Default|GetcontrollerRef)) (CallFunction|CreateDialogLines _asbase_hero) "finishedTriggerActivation"))))

(event EventBeginPlay
  (bind _asuser_input (Utilities|Casting|CastToUserInput (Game|GetPlayerController 0)))
  (Variables|Default|SetcontrollerRef _asuser_input)
  (bind _asmy_rtsgame_mode (Utilities|Casting|CastToMyRTSGameMode (Game|GetGameMode)))
  (Variables|Default|SetgameModeRef _asmy_rtsgame_mode))

(event Collision|EventActorBeginOverlap
  (params (OtherActor :type Actor%20Object%20Reference)))

(fn ConstructionScript)

(fn CreateDialogLines
  (params (heroRef :type Base%20Hero%20Object%20Reference))
  (bind _returnvalue (Class|Unit|GetGameName heroRef))
  (bind _dialoglines (LocalVariables|GetdialogLines))
  (bind _blockmessage (Variables|Default|GetblockMessage))
  (bind _dialoglines_2 (LocalVariables|GetdialogLines))
  (bind _returnvalue_2 (Utilities|Array|Length _blockmessage))
  (bind _returnvalue_3 (Utilities|String|ToString(Text) _returnvalue))
  (bind _returnvalue_4 (Utilities|String|StringToName _returnvalue_3))
  (if (> _returnvalue_2 0)
    (for _index (range 0 (- _returnvalue_2 2)) ; Inclusive
      (Utilities|Array|Add (LocalVariables|GetdialogLines) (Utilities|Struct|MakeDialogData (Utilities|Array|MakeArray (+ _index 1)) (Utilities|Array|Get(acopy) _blockmessage _index) _returnvalue_4)))
    (Utilities|Array|Add _dialoglines (Utilities|Struct|MakeDialogData (Utilities|Array|MakeArray) (Utilities|Array|Get(acopy) _blockmessage (- _returnvalue_2 1)) _returnvalue_4))
    (return _dialoglines)
    (else
      (Utilities|Array|Add _dialoglines_2 (Utilities|Struct|MakeDialogData (Utilities|Array|MakeArray) (Class|ConditionalManager|GetConditionString (Variables|/Script/MyProject.RTSGameMode|GetconditionalManager (Variables|Default|GetgameModeRef)) (Utilities|Array|MakeArray (Variables|Default|GetfailedCondition))) _returnvalue_4))
      (return _dialoglines_2))))

(fn DoesMeetConditional?
  ;[1 0.09807 0.3091] Todo: Create helper function to do this since this is common functionality
  (for _array_element (Variables|Default|Getconditions)
    (if (not (Class|ConditionalManager|GetCondition (Variables|/Script/MyProject.RTSGameMode|GetconditionalManager (Variables|Default|GetgameModeRef)) _array_element))
      (Variables|Default|SetfailedCondition _array_element)
      (return false)))
  (return true))