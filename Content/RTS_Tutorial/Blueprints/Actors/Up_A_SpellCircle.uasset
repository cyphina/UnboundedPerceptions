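; Spell circle actor that shows a rotating ground decal following the player's cursor, likely as a spell targeting indicator.
; Show scales the decal to the given radius, places it at a world location, enables Tick and plays the RotateDecal timeline, whose updates add yaw.
; Tick moves the actor to the cursor's world position.
; Hide disables Tick, hides the decal and stops the timeline; Tick also starts disabled.
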(event Custom|Show
  (params (WorldLocation :type Vector) (radius :type Float%20%28single-precision%29))
  (Actor|Tick|SetActorTickEnabled true)
  (Transformation|SetWorldScale3D (Variables|Decal|GetDecal) (Math|Vector|MakeVector 1e+02 radius radius))
  (Rendering|SetVisibility (Variables|Decal|GetDecal) true true)
  (Transformation|SetActorLocation WorldLocation false false)
  (Audio|Components|Audio|Play (Variables|Default|GetRotateDecal)))

(event Custom|Hide
  (Actor|Tick|SetActorTickEnabled false)
  (Rendering|SetVisibility (Variables|Decal|GetDecal) false true)
  (Audio|Components|Audio|Stop (Variables|Default|GetRotateDecal)))

(event EventBeginPlay
  (Actor|Tick|SetActorTickEnabled false))

(event EventTick
  (params (DeltaSeconds :type Float%20%28single-precision%29))
  (Transformation|SetActorLocation (CallFunction|GetCursorWorldPosition (Variables|Default|GetCPCRef) 8e+03) false false))

(fn ConstructionScript)