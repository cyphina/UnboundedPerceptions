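; TankMinigameStatue is a statue actor meant to launch a minigame, which is set to the drawing minigame type despite the tank name.
; Its StartMinigame function casts the game mode to MyRTSGameMode and asks its MinigameManager to start that minigame with empty triggers and parameters.
; The Interact event is an empty stub, and nothing in this Blueprint calls StartMinigame.
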(event EventBeginPlay
  (|CallParentFunction) ; This node is disabled and will not be called.\nDrag off pins to build functionality.
)

(event Collision|EventActorBeginOverlap
  (params (OtherActor :type Actor%20Object%20Reference))
  (|CallParentFunction OtherActor) ; This node is disabled and will not be called.\nDrag off pins to build functionality.
)

(event EventTick
  (params (DeltaSeconds :type Float%20%28single-precision%29))
  (|CallParentFunction DeltaSeconds) ; This node is disabled and will not be called.\nDrag off pins to build functionality.
)

(event EventInteract
  (params (hero :type Base%20Hero%20Object%20Reference)))

(fn ConstructionScript
  (|CallParentFunction))

(fn StartMinigame
  (bind _asmy_rtsgame_mode (Utilities|Casting|CastToMyRTSGameMode (Game|GetGameMode)))
  (Class|MinigameManager|StartMiniGame (Variables|/Script/MyProject.RTSGameMode|GetminigameManager _asmy_rtsgame_mode) "DrawingMiniGame" (Utilities|Struct|MakeMinigameData (Utilities|Array|MakeArray) (Utilities|Array|MakeArray) (Utilities|Array|MakeArray))))