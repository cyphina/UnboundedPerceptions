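; Area indicator actor that shows a decal sized by Radius with a ring that expands until TimeTillActivation elapses, then expires.
; Construction script and BeginPlay both orient and scale the decal, and BeginPlay also sets the actor's lifespan.
; A looping 0.01-second timer accumulates normalized progress into the ExpandTime parameter of the decal's dynamic material.
; The timer is cleared when the actor is destroyed.
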(event Custom|ExpandRing
  (Variables|Default|SetcumulativeTimeSinceSpawn (+ (Variables|Default|GetcumulativeTimeSinceSpawn) (/ 0.01 (Variables|Default|GetTimeTillActivation))))
  (Rendering|Material|SetScalarParameterValue (Variables|Default|GetdynamicMat) "ExpandTime" (Variables|Default|GetcumulativeTimeSinceSpawn) :!class /Script/Engine.MaterialInstanceDynamic))

(event EventBeginPlay
  (bind _radius (Variables|Default|GetRadius))
  (|CallParentFunction)
  (Transformation|SetWorldRotation (Variables|Default|GetDecal) "90.000000, 0, 0" false false)
  (Transformation|SetWorldScale3D (Variables|Default|GetDecal) (Math|Vector|MakeVector 1e+01 _radius _radius))
  (Actor|SetLifeSpan (Variables|Default|GetTimeTillActivation))
  (bind _returnvalue (Rendering|Material|CreateDynamicMaterialInstance (Variables|Default|GetDecal) :!class /Script/Engine.DecalComponent))
  (bind _output_get (Variables|Default|SetdynamicMat _returnvalue))
  (Rendering|Material|SetScalarParameterValue _output_get "ExpandTime" (Variables|Default|GetTimeTillActivation) :!class /Script/Engine.MaterialInstanceDynamic)
  (bind _returnvalue_2 (Utilities|Time|SetTimerbyEvent (delegate Custom|ExpandRing) 0.01 true))
  (Variables|Default|SetexpandTimer _returnvalue_2))

(event EventDestroyed
  (|CallParentFunction)
  (Utilities|Time|ClearandInvalidateTimerbyHandle (Variables|Default|GetexpandTimer)))

(fn ConstructionScript
  (bind _radius (Variables|Default|GetRadius))
  (Transformation|SetWorldRotation (Variables|Default|GetDecal) "90.000000, 0, 0" false false)
  (Transformation|SetWorldScale3D (Variables|Default|GetDecal) (Math|Vector|MakeVector 1e+01 _radius _radius)))