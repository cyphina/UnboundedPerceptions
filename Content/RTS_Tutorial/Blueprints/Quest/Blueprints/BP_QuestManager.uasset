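; Quest manager Blueprint from an RTS tutorial, holding leftover logic for marking the selected quest's current subgoal in the world.
; That logic replaces the current goal actor with a BP_GoalActor spawned at the subgoal's location, or hides the quest list's distance indicator when no location is set.
; None of it is wired to an event, so it never runs, and the construction script is empty.
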(fn ConstructionScript)